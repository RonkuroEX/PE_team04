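; BP_ProtoItem is a power-up pickup that applies an effect selected by ItemType, such as attack, speed, recovery or special attack count.
; Its construction script blocking-loads the matching mesh from the DAItemTemp data and assigns it to the Capsule mesh component.
; When player 0's pawn overlaps the Sphere, it sends ItemType through IFFItemAdhibitionMessage and destroys itself.
; Tick spins the actor by a fixed yaw step per frame, independent of delta time.
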(event OnComponentBeginOverlap(Sphere)
  (params (OverlappedComponent :type Primitive%20Component%20Object%20Reference) (OtherActor :type Actor%20Object%20Reference) (OtherComp :type Primitive%20Component%20Object%20Reference) (OtherBodyIndex :type Integer) (bFromSweep :type Boolean) (SweepResult :type Hit%20Result%20Structure%20%28by%20ref%29))
  ;[1 1 1] プレイヤーが接触した際のアイテム効果適用
  (if (== OtherActor (Game|Player|GetPlayerPawn 0))
    (Class|IFPlayer|IFFItemAdhibition(Message) (Game|Player|GetPlayerPawn 0) (Variables|Default|GetItemType))
    (Actor|DestroyActor)))

(event EventTick
  (params (DeltaSeconds :type Float%20%28single-precision%29))
  (bind _returnvalue (Transformation|GetActorRotation))
  (Transformation|SetActorRotation (Math|Rotator|MakeRotator (.roll _returnvalue) (.pitch _returnvalue) (+ (.yaw _returnvalue) 5.0))))

(fn ConstructionScript
  (bind _da_itemtemp (Variables|Default|GetDA_ItemTemp))
  (switch Utilities|FlowControl|Switch|SwitchonE_ItemType (Variables|Default|GetItemType)
    (:NewEnumerator0
      (bind _returnvalue (Utilities|LoadAssetBlocking (Variables|/Game/BP/Item/DataAsset/DA_ItemTemp.DA_ItemTemp_C|GetItemModel_ATK _da_itemtemp)))
      (bind _asstatic_mesh (Utilities|Casting|CastToStaticMesh _returnvalue))
      (Components|StaticMesh|SetStaticMesh (Variables|Default|GetCapsule) _asstatic_mesh))
    (:NewEnumerator1
      (bind _returnvalue_2 (Utilities|LoadAssetBlocking (Variables|/Game/BP/Item/DataAsset/DA_ItemTemp.DA_ItemTemp_C|GetItemModel_SPD _da_itemtemp)))
      (bind _asstatic_mesh_2 (Utilities|Casting|CastToStaticMesh _returnvalue_2))
      (Components|StaticMesh|SetStaticMesh (Variables|Default|GetCapsule) _asstatic_mesh_2))
    (:NewEnumerator2
      (bind _returnvalue_3 (Utilities|LoadAssetBlocking (Variables|/Game/BP/Item/DataAsset/DA_ItemTemp.DA_ItemTemp_C|GetItemModel_Rec _da_itemtemp)))
      (bind _asstatic_mesh_3 (Utilities|Casting|CastToStaticMesh _returnvalue_3))
      (Components|StaticMesh|SetStaticMesh (Variables|Default|GetCapsule) _asstatic_mesh_3))
    (:NewEnumerator3
      (bind _returnvalue_4 (Utilities|LoadAssetBlocking (Variables|/Game/BP/Item/DataAsset/DA_ItemTemp.DA_ItemTemp_C|GetItemModel_SPA _da_itemtemp)))
      (bind _asstatic_mesh_4 (Utilities|Casting|CastToStaticMesh _returnvalue_4))
      (Components|StaticMesh|SetStaticMesh (Variables|Default|GetCapsule) _asstatic_mesh_4))))