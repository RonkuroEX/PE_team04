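; Boss laser attack actor that stretches out as a beam and damages the player.
; While Firing, Tick lengthens the Sphere's Z scale and the Capsule's half height by fixed per-frame steps.
; BeginPlay spawns a water-ball hit effect, then clears Firing and deactivates the effect after a short delay.
; A looping timer polls Capsule overlaps and sends IFFDamageMessage to the player pawn, giving repeated damage ticks.
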(event Custom|CheckOverlap
  (Utilities|FlowControl|Sequence
    (:then_0
      (for _array_element (Collision|GetOverlappingActors (Variables|Default|GetCapsule) 0 :!class /Script/Engine.PrimitiveComponent)
        (if (== _array_element (Game|Player|GetPlayerPawn 0))
          (Class|IFPlayer|IFFDamage(Message) _array_element (Variables|Default|GetDamage%20Value) (Variables|Default|GetDamageType)))))))

(event EventTick
  (params (DeltaSeconds :type Float%20%28single-precision%29))
  (bind _sphere (Variables|Default|GetSphere))
  (bind _capsule (Variables|Default|GetCapsule))
  (if (Variables|Default|GetFiring)
    (Transformation|SetWorldScale3D _sphere (+ (Transformation|GetWorldScale _sphere) "0.000000,0.000000,0.600000"))
    (Components|Capsule|SetCapsuleHalfHeight _capsule (+ (Variables|/Script/Engine.CapsuleComponent|GetCapsuleHalfHeight _capsule) 3e+01) false)))

(event EventBeginPlay
  (Utilities|Time|SetTimerbyEvent (delegate Custom|CheckOverlap) 0.1 true)
  (bind _returnvalue (Effects|SpawnEmitteratLocation "/Game/FXVarietyPack/Particles/P_ky_waterBallHit.P_ky_waterBallHit" (Transformation|GetWorldLocation (Variables|Default|GetSphere)) "0, 0, 0" "2.000000,2.000000,2.000000"))
  (Utilities|FlowControl|Delay 0.25)
  (Variables|Default|SetFiring false)
  (Components|Activation|SetActive _returnvalue false false))

(fn ConstructionScript
  (|CallParentFunction))