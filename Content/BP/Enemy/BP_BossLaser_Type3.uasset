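; Boss laser attack that repeatedly extends a beam, then launches it along negative X.
; A looping BeginPlay sequence toggles Firing: Tick stretches Sphere and Capsule, then slides the beam and StaticMesh away before resetting to the start.
; During the slide, a timer spawns bursts of five randomly rotated accelerating bullets from StaticMesh.
; Another timer damages the player through Capsule overlaps; any damage to the actor destroys it.
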(event Custom|CheckOverlap
  (if (not (<= (.x (Transformation|GetWorldScale (Variables|Default|GetSphere))) 0.0))
    (for _array_element (Collision|GetOverlappingActors (Variables|Default|GetCapsule) 0 :!class /Script/Engine.PrimitiveComponent)
      (if (== _array_element (Game|Player|GetPlayerPawn 0))
        (Class|IFPlayer|IFFDamage(Message) _array_element (Variables|Default|GetDamage%20Value) (Variables|Default|GetDamageType))))))

(event Custom|SpawnBullets
  (bind _returnvalue (Utilities|Time|SetTimerbyEvent (delegate Custom|カスタムイベント) 0.3 true))
  (Variables|Default|SetSpawnBulletTimer _returnvalue))

(event Custom|カスタムイベント
  (CallFunction|FFireAcceleration5Way (Variables|Default|GetStaticMesh)))

(event EventTick
  (params (DeltaSeconds :type Float%20%28single-precision%29))
  (bind _sphere (Variables|Default|GetSphere))
  (bind _staticmesh (Variables|Default|GetStaticMesh))
  (bind _capsule (Variables|Default|GetCapsule))
  (bind _sphere_2 (Variables|Default|GetSphere))
  (bind _capsule_2 (Variables|Default|GetCapsule))
  (bind _returnvalue (Transformation|GetWorldLocation _staticmesh))
  (bind _returnvalue_2 (Transformation|GetWorldLocation _capsule_2))
  (bind _returnvalue_3 (Transformation|GetWorldLocation _sphere_2))
  (Transformation|SetWorldLocation _capsule_2 (Math|Vector|MakeVector (+ (* -17.0 DeltaSeconds 6e+01) (.x _returnvalue_2)) (.y _returnvalue_2) (.z _returnvalue_2)) false false)
  (if (Variables|Default|GetFiring)
    (Transformation|SetWorldScale3D _sphere (+ (Transformation|GetWorldScale _sphere) "0.000000,0.000000,0.340000"))
    (Components|Capsule|SetCapsuleHalfHeight _capsule (+ (Variables|/Script/Engine.CapsuleComponent|GetCapsuleHalfHeight _capsule) 17.0) false)
    (else
      (Transformation|SetWorldLocation _sphere_2 (Math|Vector|MakeVector (+ (* -17.0 DeltaSeconds 6e+01) (.x _returnvalue_3)) (.y _returnvalue_3) (.z _returnvalue_3)) false false)
      (Transformation|SetWorldLocation _staticmesh (Math|Vector|MakeVector (+ (* -17.0 DeltaSeconds 6e+01) (.x _returnvalue)) (.y _returnvalue) (.z _returnvalue)) false false))))

(event Game|Damage|EventAnyDamage
  (params (Damage :type Float%20%28single-precision%29) (DamageType :type Damage%20Type%20Object%20Reference) (InstigatedBy :type Controller%20Object%20Reference) (DamageCauser :type Actor%20Object%20Reference))
  (Actor|DestroyActor))

(event EventBeginPlay
  (bind _capsule (Variables|Default|GetCapsule))
  (bind _staticmesh (Variables|Default|GetStaticMesh))
  (bind _sphere (Variables|Default|GetSphere))
  (Utilities|Time|SetTimerbyEvent (delegate Custom|CheckOverlap) 0.1 true)
  (Audio|PlaySoundatLocation (Variables|Default|GetLaserSE) (Transformation|GetActorLocation) "0, 0, 0" 1.0 1.0 0.0 0 0 0 0 :!label _label)
  (Utilities|FlowControl|Delay 1.5)
  (Variables|Default|SetFiring false)
  (CallFunction|SpawnBullets)
  (Utilities|FlowControl|Delay 3.0)
  (Utilities|Time|ClearandInvalidateTimerbyHandle (Variables|Default|GetSpawnBulletTimer))
  (Utilities|FlowControl|Sequence
    (:then_0
      (Transformation|SetWorldScale3D _sphere "1.000000,1.000000,0.000000")
      (Transformation|SetWorldLocation _sphere (Variables|Default|GetStartLocation) false false))
    (:then_1
      (Components|Capsule|SetCapsuleHalfHeight _capsule 5e+01 false)
      (Transformation|SetWorldLocation _capsule (Variables|Default|GetStartLocation) false false)
      (Utilities|IsValid _staticmesh
        (:Is%20Valid
          (Transformation|SetWorldLocation _staticmesh (Variables|Default|GetStartLocation) false false)
          (Variables|Default|SetFiring true)
          (goto _label))))))

(fn ConstructionScript
  (Variables|Default|SetStartLocation (Transformation|GetWorldLocation (Variables|Default|GetCapsule))))

(fn FFireAcceleration5Way
  (params (SpawnPoint :type Scene%20Component%20Object%20Reference))
  (for _index (range 0 4)
    (Game|SpawnActorfromClass "/Game/BP/Enemy/BP_EnemyaccelerationBullet.BP_EnemyaccelerationBullet_C" (Math|Transform|MakeTransform (Transformation|GetWorldLocation SpawnPoint) (Math|Rotator|MakeRotator 0.0 0.0 (Math|Float|Lerp 0.0 3.6e+02 (Math|Random|RandomFloat))) "1.000000,1.000000,1.000000") "Undefined" "MultiplyWithRoot" 0 0.0 1.5e+03 0)))