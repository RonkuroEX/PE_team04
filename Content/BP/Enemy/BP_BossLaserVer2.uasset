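; Twin-beam boss laser attack that damages the player.
; While Firing is set, Tick stretches two spheres and two hit capsules by fixed per-frame steps, so growth is frame-rate dependent.
; A looping timer polls both capsules for the player pawn and sends IFFDamageMessage.
; BeginPlay spawns a thunder-ball emitter at each sphere, then after a short delay deactivates both and clears Firing, halting growth while damage polling continues.
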(event Custom|CheckOverlap
  (Utilities|FlowControl|Sequence
    (:then_0
      (for _array_element (Collision|GetOverlappingActors (Variables|Default|GetCapsule) 0 :!class /Script/Engine.PrimitiveComponent)
        (if (== _array_element (Game|Player|GetPlayerPawn 0))
          (Class|IFPlayer|IFFDamage(Message) _array_element (Variables|Default|GetDamage%20Value) (Variables|Default|GetDamageType)))))
    (:then_1
      (for _array_element_2 (Collision|GetOverlappingActors (Variables|Default|GetCapsule1) 0 :!class /Script/Engine.PrimitiveComponent)
        (if (== _array_element_2 (Game|Player|GetPlayerPawn 0))
          (Class|IFPlayer|IFFDamage(Message) _array_element_2 (Variables|Default|GetDamage%20Value) (Variables|Default|GetDamageType)))))))

(event EventTick
  (params (DeltaSeconds :type Float%20%28single-precision%29))
  (bind _sphere (Variables|Default|GetSphere))
  (bind _capsule1 (Variables|Default|GetCapsule1))
  (bind _sphere1 (Variables|Default|GetSphere1))
  (bind _capsule (Variables|Default|GetCapsule))
  (if (Variables|Default|GetFiring)
    (Transformation|SetWorldScale3D _sphere (+ (Transformation|GetWorldScale _sphere) "0.000000,0.000000,0.300000"))
    (Transformation|SetWorldScale3D _sphere1 (+ (Transformation|GetWorldScale _sphere1) "0.000000,0.000000,0.300000"))
    (Components|Capsule|SetCapsuleHalfHeight _capsule (+ (Variables|/Script/Engine.CapsuleComponent|GetCapsuleHalfHeight _capsule) 15.0) false)
    (Components|Capsule|SetCapsuleHalfHeight _capsule1 (+ (Variables|/Script/Engine.CapsuleComponent|GetCapsuleHalfHeight _capsule1) 15.0) false)))

(event EventBeginPlay
  (Utilities|Time|SetTimerbyEvent (delegate Custom|CheckOverlap) 0.1 true)
  (bind _returnvalue (Effects|SpawnEmitteratLocation "/Game/FXVarietyPack/Particles/P_ky_thunderBall.P_ky_thunderBall" (Transformation|GetWorldLocation (Variables|Default|GetSphere)) "0, 0, 0" "2.000000,2.000000,2.000000"))
  (bind _returnvalue_2 (Effects|SpawnEmitteratLocation "/Game/FXVarietyPack/Particles/P_ky_thunderBall.P_ky_thunderBall" (Transformation|GetWorldLocation (Variables|Default|GetSphere1)) "0, 0, 0" "2.000000,2.000000,2.000000"))
  (Utilities|FlowControl|Delay 0.5)
  (Variables|Default|SetFiring false)
  (Components|Activation|SetActive _returnvalue false false)
  (Components|Activation|SetActive _returnvalue_2 false false))

(fn ConstructionScript
  (|CallParentFunction))