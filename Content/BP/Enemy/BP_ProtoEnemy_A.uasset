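; Prototype shooter enemy A that fires spread volleys on a looping timer.
; Construction sets HP from the game instance's stage level and fire delay from its difficulty.
; Each volley's shot count grows with difficulty, spawning pairs at a box component, fanned either side of its look-at rotation with slightly uneven yaw steps.
; It extends a parent enemy, calling parent logic in construction, BeginPlay and each shot.
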(event Custom|SpawnBullet
  (CallFunction|FFireEvenWay (Utilities|Select :Index (Variables|Default|GetE_Difficulity) :NewEnumerator0 2 :NewEnumerator1 4 :NewEnumerator2 6))
  (|CallParentFunction))

(event EventBeginPlay
  (|CallParentFunction)
  (Utilities|Time|SetTimerbyEvent (delegate Custom|SpawnBullet) (Variables|Default|GetFireDelay) true))

(fn ConstructionScript
  (bind _stagelevel (Class|IFPlayerStatus|IFFGetStageLevel(Message) (Game|GetGameInstance)))
  (switch Utilities|FlowControl|Switch|SwitchonE_StageLevel _stagelevel
    (:NewEnumerator0
      (Variables|Default|SetHP 5.0))
    (:NewEnumerator1
      (Variables|Default|SetHP 1e+01))
    (:NewEnumerator2
      (Variables|Default|SetHP 15.0)))
  (bind _e_difficulity (Class|IFPlayerStatus|IFFGetDifficulity(Message) (Game|GetGameInstance)))
  (bind _output_get (Variables|Default|SetE_Difficulity _e_difficulity))
  (switch Utilities|FlowControl|Switch|SwitchonE_Difficulty _output_get
    (:NewEnumerator0
      (Variables|Default|SetFireDelay 2.0))
    (:NewEnumerator1
      (Variables|Default|SetFireDelay 1.0))
    (:NewEnumerator2
      (Variables|Default|SetFireDelay 1.0)))
  (|CallParentFunction))

(fn FFireEvenWay
  (params (Split :type Integer))
  (bind _box (Variables|Default|GetBox))
  (bind _box_2 (Variables|Default|GetBox))
  (bind _output_get (LocalVariables|SetSplitcount (/ Split 2)))
  (for _index (range 1 _output_get)
    (bind _returnvalue (CallFunction|FFindLookatRotation _box_2))
    (Game|SpawnActorfromClass "/Game/BP/Enemy/BP_Enemy_GreenBullet.BP_Enemy_GreenBullet_C" (Math|Transform|MakeTransform (Transformation|GetWorldLocation _box_2) (Math|Rotator|MakeRotator (.Roll (Math|Rotator|BreakRotator _returnvalue)) (.Pitch (Math|Rotator|BreakRotator _returnvalue)) (+ (.Yaw (Math|Rotator|BreakRotator _returnvalue)) (* (/ (/ (Variables|Default|GetSplitAngle) 2.0) 3.0) _index))) "1.000000,1.000000,1.000000") "Undefined" "MultiplyWithRoot" 0 0)
    (bind _returnvalue_2 (CallFunction|FFindLookatRotation _box))
    (Game|SpawnActorfromClass "/Game/BP/Enemy/BP_Enemy_GreenBullet.BP_Enemy_GreenBullet_C" (Math|Transform|MakeTransform (Transformation|GetWorldLocation _box) (Math|Rotator|MakeRotator (.Roll (Math|Rotator|BreakRotator _returnvalue_2)) (.Pitch (Math|Rotator|BreakRotator _returnvalue_2)) (- (.Yaw (Math|Rotator|BreakRotator _returnvalue_2)) (* (/ (/ (Variables|Default|GetSplitAngle) 2.0) 4.0) _index))) "1.000000,1.000000,1.000000") "Undefined" "MultiplyWithRoot" 0 0)))