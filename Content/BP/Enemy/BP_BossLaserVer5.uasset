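; Boss laser actor that stretches a beam and damages the player's pawn inside it.
; A looping 0.1-second timer scans the capsule's overlaps and sends IFFDamageMessage with damage value and type to the player.
; Tick lengthens the sphere's Z scale and capsule half height every frame, independent of delta time.
; Firing clears three seconds after BeginPlay; whenever it is false, the beam also narrows while still lengthening.
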(event Custom|CheckOverlap
  (for _array_element (Collision|GetOverlappingActors (Variables|Default|GetCapsule) 0 :!class /Script/Engine.PrimitiveComponent)
    (if (== _array_element (Game|Player|GetPlayerPawn 0))
      (Class|IFPlayer|IFFDamage(Message) _array_element (Variables|Default|GetDamage%20Value) (Variables|Default|GetDamageType)))))

(event EventTick
  (params (DeltaSeconds :type Float%20%28single-precision%29))
  (bind _sphere (Variables|Default|GetSphere))
  (bind _capsule (Variables|Default|GetCapsule))
  (bind _capsule_2 (Variables|Default|GetCapsule))
  (bind _sphere_2 (Variables|Default|GetSphere))
  (bind _capsule_3 (Variables|Default|GetCapsule))
  (if (Variables|Default|GetFiring)
    (Transformation|SetWorldScale3D _sphere (+ (Transformation|GetWorldScale _sphere) "0.000000,0.000000,0.340000"))
    (Components|Capsule|SetCapsuleHalfHeight _capsule (+ (Variables|/Script/Engine.CapsuleComponent|GetCapsuleHalfHeight _capsule) 17.0) false)
    (else
      (Transformation|SetWorldScale3D _sphere_2 (+ (Transformation|GetWorldScale _sphere_2) "-0.025000,-0.025000,0.340000"))
      (Components|Capsule|SetCapsuleRadius _capsule_2 (- (Variables|/Script/Engine.CapsuleComponent|GetCapsuleRadius _capsule_2) 1.3) true)
      (Utilities|IsValid _capsule_3
        (:Is%20Valid
          (Components|Capsule|SetCapsuleHalfHeight _capsule_3 (+ (Variables|/Script/Engine.CapsuleComponent|GetCapsuleHalfHeight _capsule_3) 17.0) false))))))

(event EventBeginPlay
  (Utilities|Time|SetTimerbyEvent (delegate Custom|CheckOverlap) 0.1 true)
  (Utilities|FlowControl|Delay 3.0)
  (Variables|Default|SetFiring false))

(fn ConstructionScript
  (|CallParentFunction))