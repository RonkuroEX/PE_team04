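; BP_NormalEnemy_D is a spinning enemy that sprays random blue, green or red bullets from three fire points.
; After a spawn delay, a looping timer spawns the bullets at each point's transform and calls the parent's SpawnBullet, until FEndFire clears it.
; Tick applies a constant, delta-scaled yaw spin.
; The construction script reads the GameInstance, setting HP by stage and mini-boss phase and fire interval by difficulty.
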(event Custom|FireBullet
  (CallFunction|FFireBullet (Variables|Default|GetFirePoint1))
  (CallFunction|FFireBullet (Variables|Default|GetFirePoint2))
  (CallFunction|FFireBullet (Variables|Default|GetFirePoint3))
  (|CallParentFunction))

(event EventBeginPlay
  (Utilities|FlowControl|Delay (Variables|Default|GetWaitingTime))
  (|CallParentFunction)
  (bind _returnvalue (Utilities|Time|SetTimerbyEvent (delegate Custom|FireBullet) (Variables|Default|GetFireDelay) true))
  (Variables|Default|SetFireTimer _returnvalue))

(event Collision|EventActorBeginOverlap
  (params (OtherActor :type Actor%20Object%20Reference)))

(event EventTick
  (params (DeltaSeconds :type Float%20%28single-precision%29))
  (bind _returnvalue (Transformation|GetActorRotation))
  (Transformation|SetActorRotation (Math|Rotator|MakeRotator (.roll _returnvalue) (.pitch _returnvalue) (+ (* 7.0 DeltaSeconds 6e+01) (.yaw _returnvalue)))))

(fn ConstructionScript
  (bind _beforemini_boss (Variables|Default|GetBeforeMini%20Boss))
  (|CallParentFunction)
  (bind _stagelevel (Class|IFPlayerStatus|IFFGetStageLevel(Message) (Game|GetGameInstance)))
  (switch Utilities|FlowControl|Switch|SwitchonE_StageLevel _stagelevel
    (:NewEnumerator1
      (if _beforemini_boss
        (Variables|Default|SetHP 1e+01)
        (else
          (Variables|Default|SetHP 25.0))))
    (:NewEnumerator2
      (if _beforemini_boss
        (Variables|Default|SetHP 3e+01)
        (else
          (Variables|Default|SetHP 5e+01)))))
  (bind _e_difficulity (Class|IFPlayerStatus|IFFGetDifficulity(Message) (Game|GetGameInstance)))
  (bind _output_get (Variables|Default|SetE_Difficulity _e_difficulity))
  (switch Utilities|FlowControl|Switch|SwitchonE_Difficulty _output_get
    (:NewEnumerator0
      (Variables|Default|SetFireDelay 0.7))
    (:NewEnumerator1
      (Variables|Default|SetFireDelay 0.5))
    (:NewEnumerator2
      (Variables|Default|SetFireDelay 0.3))))

(fn FFireBullet
  (params (SpawnPoint :type Scene%20Component%20Object%20Reference))
  (switch int (Math|Random|RandomInteger 3)
    (:0
      (LocalVariables|SetBullet "/Game/BP/Enemy/BP_Enemy_BlueBullet.BP_Enemy_BlueBullet_C"))
    (:1
      (LocalVariables|SetBullet "/Game/BP/Enemy/BP_Enemy_GreenBullet.BP_Enemy_GreenBullet_C"))
    (:2
      (LocalVariables|SetBullet "/Game/BP/Enemy/BP_Enemy_RedBullet.BP_Enemy_RedBullet_C")))
  (Game|SpawnActorfromClass (LocalVariables|GetBullet) (Math|Transform|MakeTransform (Transformation|GetWorldLocation SpawnPoint) (Transformation|GetWorldRotation SpawnPoint) "1.000000,1.000000,1.000000") "Undefined" "MultiplyWithRoot" 0 1e+03 1e+03 0))

(fn FEndFire
  (Utilities|Time|ClearandInvalidateTimerbyHandle (Variables|Default|GetFireTimer)))