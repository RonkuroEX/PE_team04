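; Base normal enemy that flies a spline path, optionally facing the player, and shows a lock-on widget.
; A timeline scaled by TimeLength drives movement, with EEnemyMoveType choosing a constant or pausing curve.
; Lethal damage triggers FX, score and weighted DataTable item drops; reaching the path end makes it invulnerable, then destroys it.
; EndPlay notifies the wave controller, while bullet spawning only plays sound and FEndFire is empty here.
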(event Custom|SpawnBullet
  (Audio|PlaySoundatLocation (Variables|SE|GetShotSE) (Transformation|GetActorLocation) "0, 0, 0" 1.0 1.0 0.0 0 0 0 0))

(event Custom|SplineFinished
  (CallFunction|FEndFire)
  (Variables|Default|SetInvisible true)
  (if (> (Variables|初期設定|GetWaitingTime) 0.0)
    (Utilities|FlowControl|Delay 1.5)
    (Actor|DestroyActor)
    (else
      (Actor|DestroyActor))))

(event EventBeginPlay
  (bind _targetspline (Variables|Default|GetTargetSpline))
  (Variables|Default|SetInvisible false)
  (Components|Timeline|SetPlayRate (Variables|Default|GetTimeline_Spline) (/ 1.0 (Variables|初期設定|GetTimeLength)))
  (bind (_direction _constant _pauseathalf_40_ _pauseathalf_20_ _pauseat20__50_ _pauseat20__40_ _pauseathalf_70_ _pauseatstart_70_) (Timeline|Timeline_Spline Play)
    (:Update
      (|CollapseGraph _constant _pauseathalf_40_ _pauseathalf_20_ _pauseat20__50_ _pauseat20__40_ _pauseathalf_70_ _pauseatstart_70_
        (:then
          _)
        (:then2
          _)
        (:then3
          _)
        (:then4
          _)
        (:then5
          _)
        (:then6
          _)
        (:then7
          _))
      (Utilities|FlowControl|Sequence
        (:then_0
          (Transformation|SetActorLocation (Spline|GetLocationatDistanceAlongSpline _targetspline (* (Variables|ステータス|GetTimelineValue) (Spline|GetSplineLength _targetspline)) "World") false false))
        (:then_1
          (if (Variables|Default|GetLookingPlayer)
            (Utilities|IsValid self
              (:Is%20Valid
                (Transformation|SetActorRotation (Math|Rotator|FindLookatRotation (Transformation|GetWorldLocation (Variables|Default|GetCapsule)) (Transformation|GetActorLocation (Game|Player|GetPlayerPawn 0))))))))))
    (:Finished
      (CallFunction|SplineFinished))))

(event EventIFFLock-on
  (Rendering|SetVisibility (Variables|Default|GetWidget) true false))

(event EventIFFLock-off
  (Rendering|SetVisibility (Variables|Default|GetWidget) false false))

(event Game|Damage|EventAnyDamage
  (params (Damage :type Float%20%28single-precision%29) (DamageType :type Damage%20Type%20Object%20Reference) (InstigatedBy :type Controller%20Object%20Reference) (DamageCauser :type Actor%20Object%20Reference))
  (if (not (Variables|Default|GetInvisible))
    (bind _output_get (Variables|ステータス|SetHP (- (Variables|ステータス|GetHP) Damage)))
    (if (> _output_get 0.0)
      (Audio|PlaySoundatLocation (Variables|SE|GetDamageSE) (Transformation|GetActorLocation) "0, 0, 0" 1.0 1.0 0.0 0 0 0 0)
      (else
        (CallFunction|FSpawnExplodeFX)
        (Audio|PlaySoundatLocation (Variables|SE|GetDeathSE) (Transformation|GetActorLocation) "0, 0, 0" 1.0 1.0 0.0 0 0 0 0)
        (Class|IFPlayerStatus|IFFPlusKillScore(Message) (Game|GetGameInstance) (Variables|Default|GetScore))
        (CallFunction|FItemDrop)
        (Actor|DestroyActor)))))

(event EventEndPlay
  (params (EndPlayReason :type EEndPlayReason%20Enum :default "Destroyed"))
  (CallFunction|FDecreaseMessage))

(fn ConstructionScript
  (bind _returnvalue (Actor|GetActorOfClass "/Game/Level/BP_WaveControllerBase.BP_WaveControllerBase_C"))
  (Variables|Default|SetBeforeMini%20Boss (Variables|/Game/Level/BP_WaveControllerBase.BP_WaveControllerBase_C|GetBeforeMiniBoss _returnvalue))
  (Utilities|FlowControl|Sequence
    (:then_0
      (bind _returnvalue_2 (Utilities|LoadAssetBlocking (Variables|/Game/Sound/DataAsset/Template/DA_EnemySETemp.DA_EnemySETemp_C|GetEnemyShot (Variables|SE|GetDA_EnemySE))))
      (bind _assound_cue (Utilities|Casting|CastToSoundCue _returnvalue_2))
      (Variables|SE|SetShotSE _assound_cue))
    (:then_1
      (bind _returnvalue_3 (Utilities|LoadAssetBlocking (Variables|/Game/Sound/DataAsset/Template/DA_EnemySETemp.DA_EnemySETemp_C|GetEnemyDamage (Variables|SE|GetDA_EnemySE))))
      (bind _assound_cue_2 (Utilities|Casting|CastToSoundCue _returnvalue_3))
      (Variables|SE|SetDamageSE _assound_cue_2))
    (:then_2
      (bind _returnvalue_4 (Utilities|LoadAssetBlocking (Variables|/Game/Sound/DataAsset/Template/DA_EnemySETemp.DA_EnemySETemp_C|GetEnemyDeath (Variables|SE|GetDA_EnemySE))))
      (bind _assound_cue_3 (Utilities|Casting|CastToSoundCue _returnvalue_4))
      (Variables|SE|SetDeathSE _assound_cue_3))))

(fn FChooseDropNum
  (bind _outrownames (DataTable|GetDataTableRowNames (Variables|アイテムドロップ|GetDropNumTable))) ; データテーブルの行名を取得
  (for _array_element _outrownames
    (bind _returnvalue (Utilities|GetDataTableRow (Variables|アイテムドロップ|GetDropNumTable) _array_element) ; 入れられたデータテーブルの指定の行名の情報を取得
      (:then
        (Variables|アイテムドロップ|SetTotalRate (+ (.Rate (Utilities|Struct|BreakS_DropNum _returnvalue)) (Variables|アイテムドロップ|GetTotalRate))) ; 各確率の合計値を出す
      )))
  (Variables|アイテムドロップ|SetRandomPoint (* (Math|Random|RandomFloat) (Variables|アイテムドロップ|GetTotalRate))) ; レート合計値の1倍~0倍の数値を取得する
  (bind _outrownames_2 (DataTable|GetDataTableRowNames (Variables|アイテムドロップ|GetDropNumTable)))
  (for _array_element_2 _outrownames_2
    (bind _returnvalue_2 (Utilities|GetDataTableRow (Variables|アイテムドロップ|GetDropNumTable) _array_element_2)
      (:then
        (if (< (Variables|アイテムドロップ|GetRandomPoint) (.Rate (Utilities|Struct|BreakS_DropNum _returnvalue_2))) ; アイテムレートよりランダムポイントのレートが少ないか
          (return (.Num (Utilities|Struct|BreakS_DropNum _returnvalue_2)))
          (else
            (Variables|アイテムドロップ|SetRandomPoint (- (Variables|アイテムドロップ|GetRandomPoint) (.Rate (Utilities|Struct|BreakS_DropNum _returnvalue_2)))) ; ランダムポイントからそのアイテムのレートを引いて次ループの当選率を上げる
          ))))))

(fn FChooseDropItem
  (bind _outrownames (DataTable|GetDataTableRowNames (Variables|アイテムドロップ|GetDropItemTable))) ; データテーブルの行名を取得
  (for _array_element _outrownames
    (bind _returnvalue (Utilities|GetDataTableRow (Variables|アイテムドロップ|GetDropItemTable) _array_element) ; 入れられたデータテーブルの指定の行名の情報を取得
      (:then
        (Variables|アイテムドロップ|SetTotalRate (+ (.Rate (Utilities|Struct|BreakS_DropItem _returnvalue)) (Variables|アイテムドロップ|GetTotalRate))) ; 各確率の合計値を出す
      )))
  (Variables|アイテムドロップ|SetRandomPoint (* (Math|Random|RandomFloat) (Variables|アイテムドロップ|GetTotalRate))) ; レート合計値の1倍~0倍の数値を取得する
  (bind _outrownames_2 (DataTable|GetDataTableRowNames (Variables|アイテムドロップ|GetDropItemTable)))
  (for _array_element_2 _outrownames_2
    (bind _returnvalue_2 (Utilities|GetDataTableRow (Variables|アイテムドロップ|GetDropItemTable) _array_element_2)
      (:then
        (if (< (Variables|アイテムドロップ|GetRandomPoint) (.Rate (Utilities|Struct|BreakS_DropItem _returnvalue_2))) ; アイテムレートよりランダムポイントのレートが少ないか
          (return (.Type (Utilities|Struct|BreakS_DropItem _returnvalue_2)))
          (else
            (Variables|アイテムドロップ|SetRandomPoint (- (Variables|アイテムドロップ|GetRandomPoint) (.Rate (Utilities|Struct|BreakS_DropItem _returnvalue_2)))) ; ランダムポイントからそのアイテムのレートを引いて次ループの当選率を上げる
          ))))))

(fn FSpawnExplodeFX
  (Niagara|SpawnSystematLocation (Variables|Default|GetFX_Explode) (Transformation|GetActorLocation) "0, 0, 0" "1.000000,1.000000,1.000000" true true "AutoRelease"))

(fn FFindLookatRotation
  (params (SpawnPoint :type Scene%20Component%20Object%20Reference))
  (return (Math|Rotator|FindLookatRotation (Transformation|GetWorldLocation SpawnPoint) (Transformation|GetActorLocation (Game|Player|GetPlayerPawn 0)))))

(fn FDecreaseMessage
  (bind _returnvalue (Actor|GetActorOfClass "/Game/Level/BP_WaveControllerBase.BP_WaveControllerBase_C"))
  (Class|IFStage|IFFDecreaseEnemyCount(Message) _returnvalue))

(fn FEndFire)

(fn FItemDrop
  (if (Variables|初期設定|GetDefinitelyDrop)
    (Variables|アイテムドロップ|SetTotalRate 0.0 :!label _label)
    (bind _itemtype (CallFunction|FChooseDropItem)) ; ドロップするアイテムを抽選する
    (Game|SpawnActorfromClass "/Game/BP/Item/BP_ProtoItem.BP_ProtoItem_C" (Math|Transform|MakeTransform (Transformation|GetActorLocation) "0, 0, 0" "1.000000,1.000000,1.000000") "AdjustIfPossibleButAlwaysSpawn" "OverrideRootScale" 0 _itemtype 0) ; アイテムをドロップする
    (else
      (bind _dropnum (CallFunction|FChooseDropNum))
      (if (> _dropnum 0)
        (goto _label)
        (else
          (Actor|DestroyActor))))))