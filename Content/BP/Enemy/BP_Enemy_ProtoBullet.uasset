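; BP_Enemy_ProtoBullet is an enemy projectile that damages the player pawn on capsule overlap.
; It sends value and type through an interface-style damage message, then optionally destroys itself on that hit.
; Any damage received destroys it, as does ending overlap with a Wall-tagged actor, rather than beginning it.
; The construction script applies InitialSpeed to ProjectileMovement and zeroes its speed cap, leaving the MaxSpeed variable unused.
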(event OnComponentBeginOverlap(Capsule)
  (params (OverlappedComponent :type Primitive%20Component%20Object%20Reference) (OtherActor :type Actor%20Object%20Reference) (OtherComp :type Primitive%20Component%20Object%20Reference) (OtherBodyIndex :type Integer) (bFromSweep :type Boolean) (SweepResult :type Hit%20Result%20Structure%20%28by%20ref%29))
  (if (== OtherActor (Game|Player|GetPlayerPawn 0))
    (Class|IFPlayer|IFFDamage(Message) OtherActor (Variables|Default|GetDamage%20Value) (Variables|Default|GetDamageType))
    (if (Variables|Default|GetDestroyForHit)
      (Actor|DestroyActor))))

(event OnComponentEndOverlap(Capsule)
  (params (OverlappedComponent :type Primitive%20Component%20Object%20Reference) (OtherActor :type Actor%20Object%20Reference) (OtherComp :type Primitive%20Component%20Object%20Reference) (OtherBodyIndex :type Integer))
  (CallFunction|FWallCheck OtherActor))

(event EventBeginPlay)

(event Game|Damage|EventAnyDamage
  (params (Damage :type Float%20%28single-precision%29) (DamageType :type Damage%20Type%20Object%20Reference) (InstigatedBy :type Controller%20Object%20Reference) (DamageCauser :type Actor%20Object%20Reference))
  (CallFunction|FDestoryMe))

(fn ConstructionScript
  (bind _projectilemovement (Variables|Default|GetProjectileMovement))
  (Variables|/Script/Engine.ProjectileMovementComponent|SetInitialSpeed _projectilemovement (Variables|Default|GetInitialSpeed))
  (Variables|/Script/Engine.ProjectileMovementComponent|SetMaxSpeed _projectilemovement 0.0))

(fn FDestoryMe
  (Actor|DestroyActor))

(fn FWallCheck
  (params (self2 :type Actor%20Object%20Reference))
  (if (Actor|ActorHasTag self2 "Wall")
    (CallFunction|FDestoryMe)))