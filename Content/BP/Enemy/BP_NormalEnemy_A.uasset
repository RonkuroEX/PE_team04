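; Normal enemy variant A, a child Blueprint that repeatedly fires fanned green bullets.
; Construction sets HP by stage and mini-boss phase, and fire delay by difficulty, both read from the GameInstance.
; After a wait, a looping timer spawns difficulty-scaled bullet pairs around the look-at rotation, with slightly asymmetric yaw steps, then calls the parent's SpawnBullet.
; FEndFire clears the timer.
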(event Custom|FireBullet
  (CallFunction|FFireEvenWay (Utilities|Select :Index (Variables|Default|GetE_Difficulity) :NewEnumerator0 2 :NewEnumerator1 4 :NewEnumerator2 6 :NewEnumerator3 0))
  (|CallParentFunction))

(event EventBeginPlay
  (Utilities|FlowControl|Delay (Variables|Default|GetWaitingTime))
  (|CallParentFunction)
  (bind _returnvalue (Utilities|Time|SetTimerbyEvent (delegate Custom|FireBullet) (Variables|Default|GetFireDelay) true))
  (Variables|Default|SetFireTimer _returnvalue))

(fn ConstructionScript
  (bind _beforemini_boss (Variables|Default|GetBeforeMini%20Boss))
  (|CallParentFunction)
  (bind _stagelevel (Class|IFPlayerStatus|IFFGetStageLevel(Message) (Game|GetGameInstance)))
  (switch Utilities|FlowControl|Switch|SwitchonE_StageLevel _stagelevel
    (:NewEnumerator0
      (if _beforemini_boss
        (Variables|Default|SetHP 3.0)
        (else
          (Variables|Default|SetHP 7.0))))
    (:NewEnumerator1
      (if _beforemini_boss
        (Variables|Default|SetHP 1e+01)
        (else
          (Variables|Default|SetHP 25.0))))
    (:NewEnumerator2
      (if _beforemini_boss
        (Variables|Default|SetHP 3e+01)
        (else
          (Variables|Default|SetHP 5e+01)))))
  (bind _e_difficulity (Class|IFPlayerStatus|IFFGetDifficulity(Message) (Game|GetGameInstance)))
  (bind _output_get (Variables|Default|SetE_Difficulity _e_difficulity))
  (switch Utilities|FlowControl|Switch|SwitchonE_Difficulty _output_get
    (:NewEnumerator0
      (Variables|Default|SetFireDelay 2.0))
    (:NewEnumerator1
      (Variables|Default|SetFireDelay 1.0))
    (:NewEnumerator2
      (Variables|Default|SetFireDelay 1.0))))

(fn FFireEvenWay
  (params (Split :type Integer))
  (bind _capsule (Variables|Default|GetCapsule))
  (bind _capsule_2 (Variables|Default|GetCapsule))
  (bind _output_get (LocalVariables|SetSplitcount (/ Split 2)))
  (for _index (range 1 _output_get)
    (bind _returnvalue (CallFunction|FFindLookatRotation _capsule))
    (Game|SpawnActorfromClass "/Game/BP/Enemy/BP_Enemy_GreenBullet.BP_Enemy_GreenBullet_C" (Math|Transform|MakeTransform (Transformation|GetWorldLocation _capsule) (Math|Rotator|MakeRotator (.Roll (Math|Rotator|BreakRotator _returnvalue)) (.Pitch (Math|Rotator|BreakRotator _returnvalue)) (+ (.Yaw (Math|Rotator|BreakRotator _returnvalue)) (* (/ (/ (Variables|Default|GetSplitAngle) 2.0) 3.0) _index))) "1.000000,1.000000,1.000000") "Undefined" "MultiplyWithRoot" 0 1e+03 1e+03 0)
    (bind _returnvalue_2 (CallFunction|FFindLookatRotation _capsule_2))
    (Game|SpawnActorfromClass "/Game/BP/Enemy/BP_Enemy_GreenBullet.BP_Enemy_GreenBullet_C" (Math|Transform|MakeTransform (Transformation|GetWorldLocation _capsule_2) (Math|Rotator|MakeRotator (.Roll (Math|Rotator|BreakRotator _returnvalue_2)) (.Pitch (Math|Rotator|BreakRotator _returnvalue_2)) (- (.Yaw (Math|Rotator|BreakRotator _returnvalue_2)) (* (/ (/ (Variables|Default|GetSplitAngle) 2.0) 4.0) _index))) "1.000000,1.000000,1.000000") "Undefined" "MultiplyWithRoot" 0 1e+03 1e+03 0)))

(fn FEndFire
  (Utilities|Time|ClearandInvalidateTimerbyHandle (Variables|Default|GetFireTimer)))