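; Enemy actor that periodically fires a three-shot spread at the player.
; On BeginPlay it runs the parent logic, then sets HP and fire delay from the difficulty in the player status and starts a looping timer.
; Each tick of the timer spawns a red bullet aimed at the player from the Box component, flanked by two blue bullets yawed half of SplitAngle to either side.
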(event Custom|SpawnBullet
  (bind _returnvalue (Game|Player|GetPlayerPawn 0))
  (bind _returnvalue_2 (Game|Player|GetPlayerPawn 0))
  (bind _box (Variables|Default|GetBox))
  (bind _box_2 (Variables|Default|GetBox))
  (bind _box_3 (Variables|Default|GetBox))
  (bind _returnvalue_3 (Transformation|GetActorLocation _returnvalue))
  (bind _returnvalue_4 (Transformation|GetWorldLocation _box))
  (bind _returnvalue_5 (Transformation|GetWorldLocation _box_2))
  (bind _returnvalue_6 (Transformation|GetWorldLocation _box_3))
  (bind _returnvalue_7 (Transformation|GetActorLocation _returnvalue_2))
  (bind _returnvalue_8 (Math|Rotator|FindLookatRotation _returnvalue_5 _returnvalue_3))
  (bind _returnvalue_9 (Math|Rotator|FindLookatRotation _returnvalue_6 _returnvalue_7))
  (Game|SpawnActorfromClass "/Game/BP/Enemy/BP_Enemy_RedBullet.BP_Enemy_RedBullet_C" (Math|Transform|MakeTransform _returnvalue_4 (Math|Rotator|FindLookatRotation _returnvalue_4 (Transformation|GetActorLocation (Game|Player|GetPlayerPawn 0))) "1.000000,1.000000,1.000000") "Undefined" "MultiplyWithRoot" 0 0)
  (Game|SpawnActorfromClass "/Game/BP/Enemy/BP_Enemy_BlueBullet.BP_Enemy_BlueBullet_C" (Math|Transform|MakeTransform (Transformation|GetWorldLocation (Variables|Default|GetBox)) (Math|Rotator|MakeRotator (.roll _returnvalue_8) (.pitch _returnvalue_8) (+ (.yaw _returnvalue_8) (/ (Variables|Default|GetSplitAngle) 2.0))) "1.000000,1.000000,1.000000") "Undefined" "MultiplyWithRoot" 0 0)
  (Game|SpawnActorfromClass "/Game/BP/Enemy/BP_Enemy_BlueBullet.BP_Enemy_BlueBullet_C" (Math|Transform|MakeTransform (Transformation|GetWorldLocation (Variables|Default|GetBox)) (Math|Rotator|MakeRotator (.roll _returnvalue_9) (.pitch _returnvalue_9) (- (.yaw _returnvalue_9) (/ (Variables|Default|GetSplitAngle) 2.0))) "1.000000,1.000000,1.000000") "Undefined" "MultiplyWithRoot" 0 0))

(event EventBeginPlay
  (|CallParentFunction)
  (switch Utilities|FlowControl|Switch|SwitchonE_Difficulty (Variables|/Game/Data/GI_PlayerStatus.GI_PlayerStatus_C|GetE_Difficulity (Variables|Default|GetAs%20GI%20Player%20Status))
    (:NewEnumerator0
      (Variables|Default|SetHP 5.0)
      (Variables|Default|SetFireDelay 3.0))
    (:NewEnumerator1
      (Variables|Default|SetHP 1e+01)
      (Variables|Default|SetFireDelay 2.0))
    (:NewEnumerator2
      (Variables|Default|SetHP 15.0)
      (Variables|Default|SetFireDelay 1.0)))
  (Utilities|Time|SetTimerbyEvent (delegate Custom|SpawnBullet) (Variables|Default|GetFireDelay) true))

(fn ConstructionScript
  (|CallParentFunction))