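; Boss laser hazard that emits from the left or right side, chosen by FromRight, and drifts steadily along +Y.
; A looping delay cycle resets the beam and grows it for two seconds, then stops growth for three.
; Tick stretches the sphere and capsule together while firing and pins the particle effect to the origin X.
; A repeating timer polls capsule overlaps and sends damage to the player pawn.
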(event Custom|CheckOverlap
  (for _array_element (Collision|GetOverlappingActors (Variables|Default|GetCapsule) 0 :!class /Script/Engine.PrimitiveComponent)
    (if (== _array_element (Game|Player|GetPlayerPawn 0))
      (Class|IFPlayer|IFFDamage(Message) _array_element (Variables|Default|GetDamage%20Value) (Variables|Default|GetDamageType)))))

(event EventTick
  (params (DeltaSeconds :type Float%20%28single-precision%29))
  (bind _returnvalue (Transformation|GetActorLocation))
  (bind _returnvalue_2 (Transformation|GetActorLocation))
  (bind _sphere (Variables|Default|GetSphere))
  (bind _capsule (Variables|Default|GetCapsule))
  (Transformation|SetActorLocation (Math|Vector|MakeVector (.x _returnvalue) (+ (.y _returnvalue) (* 1e+01 DeltaSeconds 6e+01)) (.z _returnvalue)) false false)
  (Transformation|SetWorldLocation (Variables|Default|GetParticleSystem) (Math|Vector|MakeVector (Variables|Default|GetDefaultLocationX) (.y _returnvalue_2) (.z _returnvalue_2)) false false)
  (if (Variables|Default|GetFiring)
    (Transformation|SetWorldScale3D _sphere (+ (Transformation|GetWorldScale _sphere) "0.000000,0.000000,0.340000"))
    (Components|Capsule|SetCapsuleHalfHeight _capsule (+ (Variables|/Script/Engine.CapsuleComponent|GetCapsuleHalfHeight _capsule) 17.0) false)))

(event EventBeginPlay
  (bind _returnvalue (Transformation|GetActorLocation))
  (Utilities|Time|SetTimerbyEvent (delegate Custom|CheckOverlap) 0.1 true)
  (Utilities|FlowControl|Delay 2.0 :!label _label)
  (Variables|Default|SetFiring false)
  (Utilities|FlowControl|Delay 3.0)
  (Transformation|SetWorldScale3D (Variables|Default|GetSphere) "1.000000,1.000000,0.000000")
  (Components|Capsule|SetCapsuleHalfHeight (Variables|Default|GetCapsule) 5e+01 false)
  (Transformation|SetActorLocation (Math|Vector|MakeVector (Variables|Default|GetDefaultLocationX) (.y _returnvalue) (.z _returnvalue)) false false)
  (Variables|Default|SetFiring true)
  (goto _label))

(fn ConstructionScript
  (|CallParentFunction)
  (if (Variables|Default|GetFromRight)
    (Variables|Default|SetDefaultLocationX 1.4e+03)
    (else
      (Variables|Default|SetDefaultLocationX -1.4e+03))))

(fn FDestoryMe)