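; BP_BossLaserCross is a boss attack actor that forms a rotating set of lasers with four particle systems.
; After a short warm-up delay, BeginPlay assigns BP_BossLaser_Type2 to two child actor components, then later clears the Spining flag and deactivates all particle systems.
; Tick advances the actor's yaw at a delta-time-scaled rate while Spining is true.
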(event EventBeginPlay
  (Utilities|FlowControl|Delay 3.0)
  (ChildActorComponent|SetChildActorClass (Variables|Default|GetChildActor) "/Game/BP/Enemy/BP_BossLaser_Type2.BP_BossLaser_Type2_C")
  (ChildActorComponent|SetChildActorClass (Variables|Default|GetChildActor1) "/Game/BP/Enemy/BP_BossLaser_Type2.BP_BossLaser_Type2_C")
  (Utilities|FlowControl|Delay 1e+01)
  (Variables|Default|SetSpining false)
  (Utilities|FlowControl|Delay 0.5)
  (Utilities|FlowControl|Sequence
    (:then_0
      (Components|Activation|Deactivate (Variables|Default|GetParticleSystem1)))
    (:then_1
      (Components|Activation|Deactivate (Variables|Default|GetParticleSystem2)))
    (:then_2
      (Components|Activation|Deactivate (Variables|Default|GetParticleSystem3)))
    (:then_3
      (Components|Activation|Deactivate (Variables|Default|GetParticleSystem)))))

(event EventTick
  (params (DeltaSeconds :type Float%20%28single-precision%29))
  (bind _returnvalue (Transformation|GetActorRotation))
  (if (Variables|Default|GetSpining)
    (Transformation|SetActorRotation (Math|Rotator|MakeRotator (.roll _returnvalue) (.pitch _returnvalue) (+ (* 0.5 DeltaSeconds 6e+01) (.yaw _returnvalue))))))

(fn ConstructionScript)