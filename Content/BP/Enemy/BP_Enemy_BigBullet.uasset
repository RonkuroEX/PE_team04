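; BP_Enemy_BigBullet is a large enemy bullet that damages the player while overlapping them.
; A looping timer started at BeginPlay polls the Capsule's overlapping actors every tenth of a second and sends IFFDamageMessage to the player pawn, so damage repeats during contact.
; It is a child Blueprint that overrides FWallCheck with an empty body and defers FDestoryMe to its parent.
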(event Custom|CheckOverlap
  (for _array_element (Collision|GetOverlappingActors (Variables|Default|GetCapsule) 0 :!class /Script/Engine.PrimitiveComponent)
    (if (== _array_element (Game|Player|GetPlayerPawn 0))
      (Class|IFPlayer|IFFDamage(Message) _array_element (Variables|Default|GetDamage%20Value) (Variables|Default|GetDamageType)))))

(event EventBeginPlay
  (Utilities|Time|SetTimerbyEvent (delegate Custom|CheckOverlap) 0.1 true))

(event EventTick
  (params (DeltaSeconds :type Float%20%28single-precision%29))
  (|CallParentFunction DeltaSeconds) ; このノードは無効になっているため呼び出せません。\n機能をビルドするにはピンをドラッグしてください。
)

(fn ConstructionScript
  (|CallParentFunction))

(fn FDestoryMe
  (|CallParentFunction))

(fn FWallCheck
  (params (self2 :type Actor%20Object%20Reference)))