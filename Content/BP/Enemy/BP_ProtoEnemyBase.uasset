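; Base enemy that travels along a target spline while facing the player and destroys itself at the end.
; A timeline scaled by TimeLength drives movement, with the move type selecting a constant or pausing curve.
; When damage depletes HP, it spawns an explosion and may drop an item, using weighted random rolls over data tables.
; It also toggles a lock-on widget, plays a shot sound on SpawnBullet and provides an aim-at-player helper.
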(event Custom|SpawnBullet
  (Audio|PlaySoundatLocation (Variables|Default|GetShotSE) (Transformation|GetActorLocation) "0, 0, 0" 1.0 1.0 0.0 0 0 0 0))

(event EventBeginPlay
  (bind _targetspline (Variables|Default|GetTargetSpline))
  (Components|Timeline|SetPlayRate (Variables|Default|GetTimeline_Spline) (/ 1.0 (Variables|Default|GetTimeLength)))
  (bind (_direction _constant _pauseathalf_40_ _pauseathalf_20_ _pauseat20__50_) (Timeline|Timeline_Spline Play)
    (:Update
      (switch Utilities|FlowControl|Switch|SwitchonE_EnemyMoveType (Variables|Default|GetE_EnemyMoveType)
        (:NewEnumerator0
          (Variables|Default|SetTimelineValue _constant))
        (:NewEnumerator1
          (Variables|Default|SetTimelineValue _pauseathalf_40_))
        (:NewEnumerator2
          (Variables|Default|SetTimelineValue _pauseathalf_20_))
        (:NewEnumerator3
          (Variables|Default|SetTimelineValue _pauseat20__50_)))
      (Transformation|SetActorTransform (Math|Transform|MakeTransform (Spline|GetLocationatDistanceAlongSpline _targetspline (* (Variables|Default|GetTimelineValue) (Spline|GetSplineLength _targetspline)) "World") (Math|Rotator|FindLookatRotation (Transformation|GetWorldLocation (Variables|Default|GetBox)) (Transformation|GetActorLocation (Game|Player|GetPlayerPawn 0))) "1.000000,1.000000,1.000000")))
    (:Finished
      (Actor|DestroyActor))))

(event EventIFFLock-on
  (Rendering|SetVisibility (Variables|Default|GetWidget) true false))

(event EventIFFLock-off
  (Rendering|SetVisibility (Variables|Default|GetWidget) false false))

(event Game|Damage|EventAnyDamage
  (params (Damage :type Float%20%28single-precision%29) (DamageType :type Damage%20Type%20Object%20Reference) (InstigatedBy :type Controller%20Object%20Reference) (DamageCauser :type Actor%20Object%20Reference))
  (bind _output_get (Variables|Default|SetHP (- (Variables|Default|GetHP) Damage)))
  (if (not (> _output_get 0.0))
    (if (Variables|Default|GetDefinitelyDrop)
      (Variables|アイテムドロップ|SetTotalRate 0.0 :!label _label)
      (bind _itemtype (CallFunction|FChooseDropItem)) ; ドロップするアイテムを抽選する
      (Game|SpawnActorfromClass "/Game/BP/Item/BP_ProtoItem.BP_ProtoItem_C" (Math|Transform|MakeTransform (Transformation|GetActorLocation) "0, 0, 0" "1.000000,1.000000,1.000000") "AdjustIfPossibleButAlwaysSpawn" "OverrideRootScale" 0 _itemtype 0) ; アイテムをドロップする
      (CallFunction|FSpawnExplodeFX)
      (Actor|DestroyActor)
      (else
        (bind _dropnum (CallFunction|FChooseDropNum))
        (if (> _dropnum 0)
          (goto _label)
          (else
            (CallFunction|FSpawnExplodeFX)
            (Actor|DestroyActor)))))))

(fn ConstructionScript
  (bind _returnvalue (Utilities|LoadAssetBlocking (Variables|/Game/BP/Enemy/DataAsset/Template/DA_EnemySETemp.DA_EnemySETemp_C|GetEnemyShot (Variables|Default|GetDA_EnemySE))))
  (bind _assound_cue (Utilities|Casting|CastToSoundCue _returnvalue))
  (Variables|Default|SetShotSE _assound_cue))

(fn FChooseDropNum
  (bind _outrownames (DataTable|GetDataTableRowNames (Variables|アイテムドロップ|GetDropNumTable))) ; データテーブルの行名を取得
  (for _array_element _outrownames
    (bind _returnvalue (Utilities|GetDataTableRow (Variables|アイテムドロップ|GetDropNumTable) _array_element) ; 入れられたデータテーブルの指定の行名の情報を取得
      (:then
        (Variables|アイテムドロップ|SetTotalRate (+ (.Rate (Utilities|Struct|BreakS_DropNum _returnvalue)) (Variables|アイテムドロップ|GetTotalRate))) ; 各確率の合計値を出す
      )))
  (Variables|アイテムドロップ|SetRandomPoint (* (Math|Random|RandomFloat) (Variables|アイテムドロップ|GetTotalRate))) ; レート合計値の1倍~0倍の数値を取得する
  (bind _outrownames_2 (DataTable|GetDataTableRowNames (Variables|アイテムドロップ|GetDropNumTable)))
  (for _array_element_2 _outrownames_2
    (bind _returnvalue_2 (Utilities|GetDataTableRow (Variables|アイテムドロップ|GetDropNumTable) _array_element_2)
      (:then
        (if (< (Variables|アイテムドロップ|GetRandomPoint) (.Rate (Utilities|Struct|BreakS_DropNum _returnvalue_2))) ; アイテムレートよりランダムポイントのレートが少ないか
          (return (.Num (Utilities|Struct|BreakS_DropNum _returnvalue_2)))
          (else
            (Variables|アイテムドロップ|SetRandomPoint (- (Variables|アイテムドロップ|GetRandomPoint) (.Rate (Utilities|Struct|BreakS_DropNum _returnvalue_2)))) ; ランダムポイントからそのアイテムのレートを引いて次ループの当選率を上げる
          ))))))

(fn FChooseDropItem
  (bind _outrownames (DataTable|GetDataTableRowNames (Variables|アイテムドロップ|GetDropItemTable))) ; データテーブルの行名を取得
  (for _array_element _outrownames
    (bind _returnvalue (Utilities|GetDataTableRow (Variables|アイテムドロップ|GetDropItemTable) _array_element) ; 入れられたデータテーブルの指定の行名の情報を取得
      (:then
        (Variables|アイテムドロップ|SetTotalRate (+ (.Rate (Utilities|Struct|BreakS_DropItem _returnvalue)) (Variables|アイテムドロップ|GetTotalRate))) ; 各確率の合計値を出す
      )))
  (Variables|アイテムドロップ|SetRandomPoint (* (Math|Random|RandomFloat) (Variables|アイテムドロップ|GetTotalRate))) ; レート合計値の1倍~0倍の数値を取得する
  (bind _outrownames_2 (DataTable|GetDataTableRowNames (Variables|アイテムドロップ|GetDropItemTable)))
  (for _array_element_2 _outrownames_2
    (bind _returnvalue_2 (Utilities|GetDataTableRow (Variables|アイテムドロップ|GetDropItemTable) _array_element_2)
      (:then
        (if (< (Variables|アイテムドロップ|GetRandomPoint) (.Rate (Utilities|Struct|BreakS_DropItem _returnvalue_2))) ; アイテムレートよりランダムポイントのレートが少ないか
          (return (.Type (Utilities|Struct|BreakS_DropItem _returnvalue_2)))
          (else
            (Variables|アイテムドロップ|SetRandomPoint (- (Variables|アイテムドロップ|GetRandomPoint) (.Rate (Utilities|Struct|BreakS_DropItem _returnvalue_2)))) ; ランダムポイントからそのアイテムのレートを引いて次ループの当選率を上げる
          ))))))

(fn FSpawnExplodeFX
  (Niagara|SpawnSystematLocation (Variables|Default|GetFX_Explode) (Transformation|GetActorLocation) "0, 0, 0" "1.000000,1.000000,1.000000" true true "AutoRelease"))

(fn FFindLookatRotation
  (params (FirePoint :type Box%20Component%20Object%20Reference))
  (return (Math|Rotator|FindLookatRotation (Transformation|GetWorldLocation FirePoint) (Transformation|GetActorLocation (Game|Player|GetPlayerPawn 0)))))