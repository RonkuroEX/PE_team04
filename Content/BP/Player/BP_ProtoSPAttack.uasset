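; BP_ProtoSPAttack is a prototype player special-attack bomb that damages actors as it expands.
; On BeginPlay a timeline grows its static mesh sharply along Y and Z while X stays fixed, then destroys the actor when finished.
; SetDamage multiplies base damage by the player's attack, and the mesh applies that damage to any actor it begins overlapping, without filtering.
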(event OnComponentBeginOverlap(StaticMesh)
  (params (OverlappedComponent :type Primitive%20Component%20Object%20Reference) (OtherActor :type Actor%20Object%20Reference) (OtherComp :type Primitive%20Component%20Object%20Reference) (OtherBodyIndex :type Integer) (bFromSweep :type Boolean) (SweepResult :type Hit%20Result%20Structure%20%28by%20ref%29))
  (Game|Damage|ApplyDamage OtherActor (Variables|Default|GetBomDanage) 0 0))

(event Custom|SetDamage
  (params (PlayerATK :type Float%20%28double-precision%29))
  (Variables|Default|SetBomDanage (* (Variables|Default|GetBaseDamage) PlayerATK)) ; ベースダメージ×プレイヤーの攻撃力が最終的なボムのダメージになります
)

(event EventBeginPlay
  (bind _bomscale (Timeline|Timeline_BomScale PlayFromStart)
    (:Update
      (Transformation|SetWorldScale3D (Variables|Default|GetStaticMesh) (Math|Vector|MakeVector 1.0 (Math|Float|Lerp 0.5 4e+01 _bomscale) (Math|Float|Lerp 0.5 4e+01 _bomscale))))
    (:Finished
      (Actor|DestroyActor))))

(fn ConstructionScript)