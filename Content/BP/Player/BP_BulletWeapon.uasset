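; Player weapon that fires bullets and missiles on an interface fire call, scaling its pattern with WayLevel.
; A fire-delay gate drives FireLoop, where higher levels add muzzles, twin center shots and angled split side shots.
; At top levels, MissileLoop launches paired high-damage missiles on its own cooldown, targeting Enemy-tagged actors by stored minimum distance and sending lock-on/off messages.
; Construction loads both sounds from a data asset.
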(event Custom|FireLoop
  (bind _player_atk (Variables|Default|GetPlayer%20ATK))
  (bind _player_atk_2 (Variables|Default|GetPlayer%20ATK))
  (bind _player_atk_3 (Variables|Default|GetPlayer%20ATK))
  (bind _muzzle_level2_left (Variables|Default|Getmuzzle_Level2_Left))
  (bind _muzzle_level2_right (Variables|Default|Getmuzzle_Level2_Right))
  (bind _player_atk_4 (Variables|Default|GetPlayer%20ATK))
  (bind _muzzle_level3_left (Variables|Default|Getmuzzle_Level3_Left))
  (bind _muzzle_level3_right (Variables|Default|Getmuzzle_Level3_Right))
  (bind _muzzle_level1 (Variables|Default|Getmuzzle_Level1))
  (bind _player_atk_5 (Variables|Default|GetPlayer%20ATK))
  (Audio|PlaySoundatLocation (Variables|Default|GetSE_Shot) (Transformation|GetActorLocation) "0, 0, 0" 1.0 1.0 0.0 0 0 0 0)
  (if (>= (Variables|Default|GetWay%20Level) 4)
    (CallFunction|FSpawnBulletTwin _muzzle_level1 _player_atk_5)
    (else
      (CallFunction|FSpawnBullet _muzzle_level1 _player_atk_5 false 0.0)))
  (if (>= (Variables|Default|GetWay%20Level) 2)
    (if (>= (Variables|Default|GetWay%20Level) 5)
      (CallFunction|FSpawnBullet _muzzle_level2_left _player_atk_2 true 1e+01)
      (CallFunction|FSpawnBullet _muzzle_level2_right _player_atk_3 true 1e+01)
      (else
        (CallFunction|FSpawnBullet _muzzle_level2_left _player_atk_2 false 0.0)
        (CallFunction|FSpawnBullet _muzzle_level2_right _player_atk_3 false 0.0)))
    (if (>= (Variables|Default|GetWay%20Level) 3)
      (if (>= (Variables|Default|GetWay%20Level) 6)
        (CallFunction|FSpawnBullet _muzzle_level3_left _player_atk true 2e+01)
        (CallFunction|FSpawnBullet _muzzle_level3_right _player_atk_4 true 2e+01)
        (else
          (CallFunction|FSpawnBullet _muzzle_level3_left _player_atk false 0.0)
          (CallFunction|FSpawnBullet _muzzle_level3_right _player_atk_4 false 0.0))))))

(event Custom|MissileLoop
  (bind _targetactor (Variables|Default|GetTargetActor))
  (if (>= (Variables|Default|GetWay%20Level) 7)
    (Utilities|FlowControl|DoOnce false :!label _label
      (:Completed
        (Audio|PlaySoundatLocation (Variables|Default|GetSE_Missile) (Transformation|GetActorLocation) "0, 0, 0" 1.0 1.0 0.0 0 0 0 0)
        (Utilities|IsValid _targetactor
          (:Is%20Valid
            (Class|IFEnemy|IFFLock-off(Message) _targetactor))
          (:Is%20Not%20Valid
            _))
        (CallFunction|FSetMissileTarget)
        (CallFunction|FSpawnMissile (Variables|Default|GetMissileLauncher_Left) (* (Variables|Default|GetPlayer%20ATK) 5.0))
        (CallFunction|FSpawnMissile (Variables|Default|GetMissileLauncher_Right) (* (Variables|Default|GetPlayer%20ATK) 5.0))
        (Utilities|FlowControl|Delay 1.5)
        (goto _label Reset)))))

(event EventIFFFire
  (params (PlayerATK :type Float%20%28double-precision%29) (FireDelay :type Float%20%28double-precision%29) (WayLevel :type Integer))
  (Variables|Default|SetPlayer%20ATK PlayerATK)
  (Variables|Default|SetWay%20Level WayLevel)
  (Utilities|FlowControl|DoOnce false :!label _label
    (:Completed
      (CallFunction|FireLoop)
      (CallFunction|MissileLoop)
      (Utilities|FlowControl|Delay FireDelay)
      (goto _label Reset))))

(fn ConstructionScript
  (bind _da_wepon (Variables|Default|GetDA_Wepon))
  (Utilities|FlowControl|Sequence
    (:then_0
      (bind _returnvalue (Utilities|LoadAssetBlocking (Variables|/Game/BP/Player/DataAsset/DA_WeponTemp.DA_WeponTemp_C|GetSE_shot _da_wepon)))
      (bind _assound_cue (Utilities|Casting|CastToSoundCue _returnvalue))
      (Variables|Default|SetSE_Shot _assound_cue))
    (:then_1
      (bind _returnvalue_2 (Utilities|LoadAssetBlocking (Variables|/Game/BP/Player/DataAsset/DA_WeponTemp.DA_WeponTemp_C|GetSE_Missile _da_wepon)))
      (bind _assound_cue_2 (Utilities|Casting|CastToSoundCue _returnvalue_2))
      (Variables|Default|SetSE_Missile _assound_cue_2))))

(fn FSpawnBullet
  (params (muzzul :type Static%20Mesh%20Component%20Object%20Reference) (ATK :type Float%20%28double-precision%29) (Split :type Boolean) (SpritAngle :type Float%20%28double-precision%29))
  (bind _returnvalue (Transformation|GetWorldLocation muzzul))
  (LocalVariables|SetLocal_ATK ATK)
  (LocalVariables|SetLocal_SpritAngle SpritAngle)
  (if Split
    (Game|SpawnActorfromClass "/Game/BP/Player/BP_ProtoBullet.BP_ProtoBullet_C" (Math|Transform|MakeTransform _returnvalue (Math|Rotator|MakeRotator 0.0 0.0 (LocalVariables|GetLocal_SpritAngle)) "1.000000,1.000000,1.000000") "AlwaysSpawn" "MultiplyWithRoot" 0 (LocalVariables|GetLocal_ATK) 0)
    (Math|Float|NegateFloat (LocalVariables|GetLocal_SpritAngle)
      (:%20%20
        (Game|SpawnActorfromClass "/Game/BP/Player/BP_ProtoBullet.BP_ProtoBullet_C" (Math|Transform|MakeTransform _returnvalue (Math|Rotator|MakeRotator 0.0 0.0 (LocalVariables|GetLocal_SpritAngle)) "1.000000,1.000000,1.000000") "AlwaysSpawn" "MultiplyWithRoot" 0 (LocalVariables|GetLocal_ATK) 0)))
    (else
      (Game|SpawnActorfromClass "/Game/BP/Player/BP_ProtoBullet.BP_ProtoBullet_C" (Math|Transform|MakeTransform _returnvalue "0, 0, 0" "1.000000,1.000000,1.000000") "AlwaysSpawn" "MultiplyWithRoot" 0 (LocalVariables|GetLocal_ATK) 0))))

(fn FSpawnMissile
  (params (Launcher :type Static%20Mesh%20Component%20Object%20Reference) (ATK :type Float%20%28double-precision%29))
  (bind _returnvalue (Transformation|GetWorldLocation Launcher))
  (bind _targetactor (Variables|Default|GetTargetActor))
  (Game|SpawnActorfromClass "/Game/BP/Player/BP_Missile.BP_Missile_C" (Math|Transform|MakeTransform (Math|Vector|MakeVector (.x _returnvalue) (.y _returnvalue) 0.0) (Math|Rotator|MakeRotator 0.0 0.0 (.yaw (Transformation|GetWorldRotation Launcher))) "1.000000,1.000000,1.000000") "AlwaysSpawn" "MultiplyWithRoot" 0 ATK (Variables|Default|GetTargetActor) 0)
  (Utilities|IsValid _targetactor
    (:Is%20Valid
      (Class|IFEnemy|IFFLock-on(Message) _targetactor))))

(fn FSetMissileTarget
  (bind _outactors (Actor|GetAllActorswithTag "Enemy"))
  (for _array_element _outactors
    (if (< (Transformation|GetDistanceTo _array_element self) (LocalVariables|GetMinDistance))
      (LocalVariables|SetMinDistance (Transformation|GetDistanceTo _array_element self))
      (Variables|Default|SetTargetActor _array_element))))

(fn FSpawnBulletTwin
  (params (mazzul :type Static%20Mesh%20Component%20Object%20Reference) (ATK :type Float%20%28double-precision%29))
  (bind _returnvalue (Transformation|GetWorldLocation mazzul))
  (Game|SpawnActorfromClass "/Game/BP/Player/BP_ProtoBullet.BP_ProtoBullet_C" (Math|Transform|MakeTransform (Math|Vector|MakeVector (+ (.x _returnvalue) 25.0) (.y _returnvalue) (.z _returnvalue)) "0, 0, 0" "1.000000,1.000000,1.000000") "AlwaysSpawn" "MultiplyWithRoot" 0 ATK 0)
  (Game|SpawnActorfromClass "/Game/BP/Player/BP_ProtoBullet.BP_ProtoBullet_C" (Math|Transform|MakeTransform (Math|Vector|MakeVector (- (.x _returnvalue) 25.0) (.y _returnvalue) (.z _returnvalue)) "0, 0, 0" "1.000000,1.000000,1.000000") "AlwaysSpawn" "MultiplyWithRoot" 0 ATK 0))