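; Player pawn for a shooter, with spline entry, movement, weapon-rack firing, timed items, invincible special attack and mesh by WayLevel.
; Damage, including self-inflicted vaccine shots, banks hits by bullet type and applies HP-based debuffs to attack, fire delay and speed.
; After a delay, timer-driven "super recovery" refills HP.
; Recovery milestones buff GI_PlayerStatus stats by damage severity, and full recovery also spends the banked hits as bonuses.
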(event Custom|SuperRecovery
  (bind _proto_game_instance (Variables|Default|GetProto%20Game%20Instance))
  ;[0.17 1 0.1489] 一定時間後に超回復を発生させる
  (bind _returnvalue (Utilities|Time|SetTimerbyFunctionName 0 "カスタムイベント" 0.1 true))
  (Variables|タイマー|SetRecoveryTimer _returnvalue)
  (Variables|計算用|SetRiperdHP 0.0)
  (Variables|計算用|SetLostHP (- 1e+02 (Variables|ステータス|GetHP)))
  (Variables|計算用|SetFormerStatus (Utilities|Array|MakeArray (Variables|/Game/Data/GI_PlayerStatus.GI_PlayerStatus_C|GetPlayer_ATK _proto_game_instance) (Variables|/Game/Data/GI_PlayerStatus.GI_PlayerStatus_C|GetPlayer_SPD _proto_game_instance) (Variables|/Game/Data/GI_PlayerStatus.GI_PlayerStatus_C|GetPlayer_SubReac _proto_game_instance)))
  (Components|Capsule|SetCapsuleSize (Variables|Default|GetHitBox) 3e+01 45.0 true)
  (Variables|Default|SetBuffLevel 0)
  (Development|PrintString "回復開始！" true true "(R=0.000000,G=1.000000,B=0.117673,A=1.000000)"))

(event Custom|Debuff
  ;[1 0.225 0.9363] デバフ管理
  (CallFunction|FCheckSeverityOfDamage)
  (Variables|バフ・デバフ|SetDebuff_Volume (Utilities|Select :Index (Variables|ステータス|GetSeverityDamage) :NewEnumerator0 0.0 :NewEnumerator1 0.25 :NewEnumerator2 0.5 :NewEnumerator3 0.75 :NewEnumerator4 0.9)))

(event Custom|カスタムイベント
  (Variables|計算用|SetRiperdHP (+ (Variables|計算用|GetRiperdHP) 1.0))
  (Variables|ステータス|SetHP (+ (Variables|ステータス|GetHP) 1.0))
  (CallFunction|Debuff)
  (Utilities|BuffCheck
    (:NewParam
      (if (>= (Variables|ステータス|GetHP) (Variables|/Game/Data/GI_PlayerStatus.GI_PlayerStatus_C|GetPlayer_HP (Variables|Default|GetProto%20Game%20Instance)))
        (Variables|ステータス|SetHP (Variables|/Game/Data/GI_PlayerStatus.GI_PlayerStatus_C|GetPlayer_HP (Variables|Default|GetProto%20Game%20Instance)))
        (Utilities|Time|ClearandInvalidateTimerbyHandle (Variables|タイマー|GetRecoveryTimer))
        (Development|PrintString "回復完了！" true true "(R=0.008359,G=1.000000,B=0.083694,A=1.000000)")))))

(event Custom|Recover
  (params (RecoveryTime :type Float%20%28double-precision%29))
  ;[0.17 1 0.1489] 一定時間後に超回復を発生させる
  (bind _returnvalue (Utilities|Time|SetTimerbyEvent (delegate Custom|SuperRecovery) RecoveryTime))
  (Variables|タイマー|SetRecoveryWaitTimer _returnvalue))

(event Input|EnhancedActionEvents|EnhancedInputActionIA_SPAttack
  (params (ActionValue :type Boolean) (ElapsedSeconds :type Float%20%28double-precision%29) (TriggeredSeconds :type Float%20%28double-precision%29) (InputAction :type Input%20Action%20Object%20Reference :default "/Game/Input/Shooting/IA_SPAttack.IA_SPAttack"))
  (bind _spattackcount (Variables|ステータス|GetSPAttackCount))
  ;[1 0.1896 0.1916] 必殺技発動
  (Utilities|FlowControl|DoOnce false :!label _label
    (:Completed
      (if (> _spattackcount 0)
        (Math|Integer|DecrementInt _spattackcount
          (:%20%20
            (Class|IFGamemode|IFFItem(Message) (Game|GetGameMode) "NewEnumerator3" 0.0)
            (Variables|Default|Setinvincible true)
            (Game|SpawnActorfromClass "/Game/BP/Player/BP_ProtoSPAttack1.BP_ProtoSPAttack1_C" (Math|Transform|MakeTransform "0.000000,50.000000,0.000000" "0, 0, 0" "1.000000,1.000000,1.000000") "Undefined" "MultiplyWithRoot" 0 (Variables|/Game/Data/GI_PlayerStatus.GI_PlayerStatus_C|GetPlayer_ATK (Variables|Default|GetProto%20Game%20Instance)) 0)
            (Utilities|FlowControl|Delay 5.0)
            (Variables|Default|Setinvincible false)
            (goto _label Reset)))
        (else
          (Development|PrintString "必殺技の弾数が足りないです！" true true "(R=1.000000,G=0.000000,B=0.079394,A=1.000000)")
          (Utilities|FlowControl|Delay 3.0)
          (goto _label Reset))))))

(event Input|EnhancedActionEvents|EnhancedInputActionIA_Vaccine
  (params (ActionValue :type Boolean) (ElapsedSeconds :type Float%20%28double-precision%29) (TriggeredSeconds :type Float%20%28double-precision%29) (InputAction :type Input%20Action%20Object%20Reference :default "/Game/Input/Shooting/IA_Vaccine.IA_Vaccine"))
  (bind _proto_game_instance (Variables|Default|GetProto%20Game%20Instance))
  (bind _player_subreac (Variables|/Game/Data/GI_PlayerStatus.GI_PlayerStatus_C|GetPlayer_SubReac _proto_game_instance))
  ;[1 0.2058 0.8832] ワクチン投与（自傷ダメージ）
  (:Started
    (if (Variables|Default|Getinvincible)
      (Development|PrintString "無敵状態でワクチンは使えなくなっています" true true "(R=1.000000,G=0.112500,B=0.112500,A=1.000000)")
      (else
        (CallFunction|IFFDamage 25.0 "NewEnumerator4")
        (Components|Capsule|SetCapsuleSize (Variables|Default|GetHitBox) (* (Variables|/Game/Data/GI_PlayerStatus.GI_PlayerStatus_C|GetDefaultHitRadius _proto_game_instance) _player_subreac) (* _player_subreac (Variables|/Game/Data/GI_PlayerStatus.GI_PlayerStatus_C|GetDefaultHitHHeight _proto_game_instance)) true)))))

(event Input|EnhancedActionEvents|EnhancedInputActionIA_Fire
  (params (ActionValue :type Float%20%28double-precision%29) (ElapsedSeconds :type Float%20%28double-precision%29) (TriggeredSeconds :type Float%20%28double-precision%29) (InputAction :type Input%20Action%20Object%20Reference :default "/Game/Input/Shooting/IA_Fire.IA_Fire"))
  ;[1 0.2869 0.2012] 弾の射撃
  (Class|IFWeapon|IFFFire(Message) (Variables|/Script/Engine.ChildActorComponent|GetChildActor (Variables|Default|GetWeaponRack)) (- (* (Variables|/Game/Data/GI_PlayerStatus.GI_PlayerStatus_C|GetPlayer_ATK (Variables|Default|GetProto%20Game%20Instance)) (Variables|バフ・デバフ|GetItemATKBuff_Volume)) (* (Variables|/Game/Data/GI_PlayerStatus.GI_PlayerStatus_C|GetPlayer_ATK (Variables|Default|GetProto%20Game%20Instance)) (Variables|バフ・デバフ|GetDebuff_Volume))) (+ (Variables|/Game/Data/GI_PlayerStatus.GI_PlayerStatus_C|GetPlayer_FireDelay (Variables|Default|GetProto%20Game%20Instance)) (* (Variables|/Game/Data/GI_PlayerStatus.GI_PlayerStatus_C|GetPlayer_FireDelay (Variables|Default|GetProto%20Game%20Instance)) (Variables|バフ・デバフ|GetDebuff_Volume))) (Variables|/Game/Data/GI_PlayerStatus.GI_PlayerStatus_C|GetWayLevel (Variables|Default|GetProto%20Game%20Instance))))

(event Input|EnhancedActionEvents|EnhancedInputActionIA_MoveVer
  (params (ActionValue :type Float%20%28double-precision%29) (ElapsedSeconds :type Float%20%28double-precision%29) (TriggeredSeconds :type Float%20%28double-precision%29) (InputAction :type Input%20Action%20Object%20Reference :default "/Game/Input/Shooting/IA_MoveVer.IA_MoveVer"))
  ;[1 0.8292 0.3282] 上下左右移動
  (bind _returnvalue (CallFunction|FMoveCal ActionValue))
  (Transformation|SetActorLocation (+ (Transformation|GetActorLocation) (Math|Vector|NegateVector (Math|Vector|MakeVector 0.0 _returnvalue 0.0))) true false))

(event Input|EnhancedActionEvents|EnhancedInputActionIA_MoveHori
  (params (ActionValue :type Float%20%28double-precision%29) (ElapsedSeconds :type Float%20%28double-precision%29) (TriggeredSeconds :type Float%20%28double-precision%29) (InputAction :type Input%20Action%20Object%20Reference :default "/Game/Input/Shooting/IA_MoveHori.IA_MoveHori"))
  ;[1 0.8292 0.3282] 上下左右移動
  (:Triggered
    (bind _returnvalue (CallFunction|FMoveCal ActionValue))
    (Transformation|SetActorLocation (+ (Transformation|GetActorLocation) (Math|Vector|NegateVector (Math|Vector|MakeVector _returnvalue 0.0 0.0))) true false)
    (Transformation|SetActorRotation (Math|Rotator|MakeRotator 0.0 (Math|Float|Lerp 0.0 45.0 ActionValue) 0.0)))
  (:Completed
    (Transformation|SetActorRotation "0, 0, 0")))

(event EventIFFModelChange
  (params (WayLevel :type Integer))
  (bind _da_player (Variables|Default|GetDA_Player))
  (switch int WayLevel
    (:Default
      (bind _returnvalue (Utilities|LoadAssetBlocking (Variables|/Game/BP/Player/DataAsset/DA_PlayerTemp.DA_PlayerTemp_C|GetPlayerModel_Way5 _da_player) :!label _label))
      (bind _asstatic_mesh (Utilities|Casting|CastToStaticMesh _returnvalue))
      (Components|StaticMesh|SetStaticMesh (Variables|Default|GetProtoPrayerBody) _asstatic_mesh))
    (:1
      (bind _returnvalue_2 (Utilities|LoadAssetBlocking (Variables|/Game/BP/Player/DataAsset/DA_PlayerTemp.DA_PlayerTemp_C|GetPlayerModel_Way1 _da_player)))
      (bind _asstatic_mesh_2 (Utilities|Casting|CastToStaticMesh _returnvalue_2))
      (Components|StaticMesh|SetStaticMesh (Variables|Default|GetProtoPrayerBody) _asstatic_mesh_2))
    (:2
      (bind _returnvalue_3 (Utilities|LoadAssetBlocking (Variables|/Game/BP/Player/DataAsset/DA_PlayerTemp.DA_PlayerTemp_C|GetPlayerModel_Way3 _da_player)))
      (bind _asstatic_mesh_3 (Utilities|Casting|CastToStaticMesh _returnvalue_3))
      (Components|StaticMesh|SetStaticMesh (Variables|Default|GetProtoPrayerBody) _asstatic_mesh_3))
    (:3
      (goto _label))))

(event EventIFFItemAdhibition
  (params (ItemType :type E_ItemType%20Enum :default "NewEnumerator0"))
  (bind _spattackcount (Variables|ステータス|GetSPAttackCount))
  ;[1 0.4794 0.2048] アイテムの効果発動
  (switch Utilities|FlowControl|Switch|SwitchonE_ItemType ItemType
    (:NewEnumerator0
      (Variables|バフ・デバフ|SetItemATKBuff_Volume 1.5)
      (Class|IFGamemode|IFFItem(Message) (Game|GetGameMode) ItemType (Variables|タイマー|GetItemTime))
      (Utilities|FlowControl|RetriggerableDelay (Variables|タイマー|GetItemTime))
      (Variables|バフ・デバフ|SetItemATKBuff_Volume 1.0))
    (:NewEnumerator1
      (Variables|バフ・デバフ|SetItemSpeedBuff_Volume 1.5)
      (Class|IFGamemode|IFFItem(Message) (Game|GetGameMode) ItemType (Variables|タイマー|GetItemTime))
      (Utilities|FlowControl|RetriggerableDelay (Variables|タイマー|GetItemTime))
      (Variables|バフ・デバフ|SetItemSpeedBuff_Volume 1.0))
    (:NewEnumerator2
      (Variables|ステータス|SetRecoveryTime (/ (Variables|ステータス|GetRecoveryTime) 2.0))
      (Class|IFGamemode|IFFItem(Message) (Game|GetGameMode) ItemType (Variables|タイマー|GetItemTime))
      (if (Utilities|Time|IsTimerActivebyHandle (Variables|タイマー|GetRecoveryWaitTimer))
        (CallFunction|Recover (/ (Utilities|Time|GetTimerRemainingTimebyHandle (Variables|タイマー|GetRecoveryWaitTimer)) 2.0)))
      (Utilities|FlowControl|RetriggerableDelay (Variables|タイマー|GetItemTime))
      (Variables|ステータス|SetRecoveryTime (.RecoveryTime (Utilities|GetClassDefaults "BP_ProtoPlayer_C"))))
    (:NewEnumerator3
      (if (< _spattackcount 5)
        (Math|Integer|IncrementInt _spattackcount
          (:%20%20
            (Class|IFGamemode|IFFItem(Message) (Game|GetGameMode) ItemType 0.0)
            (Components|StaticMesh|SetStaticMesh (Variables|Default|GetProtoPrayerBody) "/Game/BP/Player/Model/Playerway5.Playerway5")))))))

(event EventIFFDamage
  (params (DamageValue :type Float%20%28double-precision%29) (DamageType :type E_DamageType%20Enum :default "NewEnumerator0"))
  ;[1 0.2067 0.8354] 被ダメージ時の処理
  (if (not (Variables|Default|Getinvincible))
    (Default|DamageTypeCheck (Variables|Default|GetProto%20Game%20Instance) DamageType)
    (switch Utilities|FlowControl|Switch|SwitchonE_DamageType DamageType
      (:NewEnumerator0
        (Math|Integer|IncrementInt (Variables|計算用|GetRedBulletStock)
          (:%20%20
            _)))
      (:NewEnumerator1
        (Math|Integer|IncrementInt (Variables|計算用|GetBlueBulletStock)
          (:%20%20
            _)))
      (:NewEnumerator2
        (Math|Integer|IncrementInt (Variables|計算用|GetGreenBulletStock)
          (:%20%20
            _)))
      (:NewEnumerator3
        (Math|Integer|IncrementInt (Variables|計算用|GetSpecialAttackStock)
          (:%20%20
            _)))
      (:NewEnumerator4
        _))
    (bind _output_get (Variables|ステータス|SetHP (- (Variables|ステータス|GetHP) DamageValue)))
    (if (<= _output_get 0.0)
      ;;[1 1 1] ゲームオーバー
      (Rendering|SetVisibility (Variables|Default|GetProtoPrayerBody) false false)
      (Collision|SetCollisionEnabled (Variables|Default|GetHitBox) "NoCollision")
      (Class|IFPlayerController|IFFChangeIAC(Message) (Game|GetPlayerController 0))
      (Class|IFGamemode|IFFGameOver(Message) (Game|GetGameMode))
      (Utilities|Time|ClearandInvalidateTimerbyHandle (Variables|タイマー|GetRecoveryWaitTimer))
      (else
        (Utilities|Time|ClearandInvalidateTimerbyHandle (Variables|タイマー|GetRecoveryTimer))
        (CallFunction|Debuff)
        (CallFunction|Recover (Variables|ステータス|GetRecoveryTime))))))

(event EventPossessed
  (params (NewController :type Controller%20Object%20Reference))
  (bind _returnvalue (Actor|GetActorOfClass "/Game/BP/Enemy/BP_MoveSpline.BP_MoveSpline_C"))
  (Variables|Default|SetAdmissionSpline (Actor|GetComponentbyClass _returnvalue "/Script/Engine.SplineComponent"))
  (bind _新規track_0 (Timeline|タイムライン Play)
    (:Update
      (Transformation|SetActorTransform (Math|Transform|MakeTransform (Spline|GetLocationatDistanceAlongSpline (Variables|Default|GetAdmissionSpline) (* _新規track_0 (Spline|GetSplineLength (Variables|Default|GetAdmissionSpline))) "World") "0, 0, 0" "1.000000,1.000000,1.000000")))))

(fn ConstructionScript
  (bind _asgi_player_status (Utilities|Casting|CastToGI_PlayerStatus (Game|GetGameInstance)))
  (bind _output_get (Variables|Default|SetProto%20Game%20Instance _asgi_player_status))
  (Variables|ステータス|SetHP (Variables|/Game/Data/GI_PlayerStatus.GI_PlayerStatus_C|GetPlayer_HP _output_get))
  (CallFunction|IFFModelChange (Variables|/Game/Data/GI_PlayerStatus.GI_PlayerStatus_C|GetWayLevel (Variables|Default|GetProto%20Game%20Instance)))
  (Components|Capsule|SetCapsuleSize (Variables|Default|GetHitBox) (Variables|/Game/Data/GI_PlayerStatus.GI_PlayerStatus_C|GetDefaultHitRadius (Variables|Default|GetProto%20Game%20Instance)) (Variables|/Game/Data/GI_PlayerStatus.GI_PlayerStatus_C|GetDefaultHitHHeight (Variables|Default|GetProto%20Game%20Instance)) true))

(fn FCheckSeverityOfDamage
  (bind _proto_game_instance (Variables|Default|GetProto%20Game%20Instance))
  (bind _player_hp (Variables|/Game/Data/GI_PlayerStatus.GI_PlayerStatus_C|GetPlayer_HP _proto_game_instance))
  (if (<= (Variables|ステータス|GetHP) (* _player_hp 0.1))
    (Variables|ステータス|SetSeverityDamage "NewEnumerator4")
    (elif (<= (Variables|ステータス|GetHP) (* _player_hp 0.25))
      (Variables|ステータス|SetSeverityDamage "NewEnumerator3")
      (elif (<= (Variables|ステータス|GetHP) (* _player_hp 0.5))
        (Variables|ステータス|SetSeverityDamage "NewEnumerator2")
        (elif (<= (Variables|ステータス|GetHP) (* _player_hp 0.75))
          (Variables|ステータス|SetSeverityDamage "NewEnumerator1")
          (else
            (Variables|ステータス|SetSeverityDamage "NewEnumerator0")))))))

(fn FBuff*cal
  (params (Applicable%20to :type Float%20%28double-precision%29%20%28by%20ref%29) (FormerStatus :type Float%20%28double-precision%29))
  (|SetBy-RefVar Applicable%20to (* FormerStatus (Variables|バフ・デバフ|GetBuff_Volume))))

(fn FBuff/cal
  (params (Applicable%20to :type Float%20%28double-precision%29%20%28by%20ref%29) (FormerStatus :type Float%20%28double-precision%29))
  (|SetBy-RefVar Applicable%20to (/ FormerStatus (Variables|バフ・デバフ|GetBuff_Volume))))

(fn FBuffALLapply
  (CallFunction|FBuff*cal (Variables|/Game/Data/GI_PlayerStatus.GI_PlayerStatus_C|GetPlayer_ATK (Variables|Default|GetProto%20Game%20Instance)) (Utilities|Array|Get(acopy) (Variables|計算用|GetFormerStatus)))
  (CallFunction|FBuff*cal (Variables|/Game/Data/GI_PlayerStatus.GI_PlayerStatus_C|GetPlayer_SPD (Variables|Default|GetProto%20Game%20Instance)) (Utilities|Array|Get(acopy) (Variables|計算用|GetFormerStatus) 1))
  (CallFunction|FBuff/cal (Variables|/Game/Data/GI_PlayerStatus.GI_PlayerStatus_C|GetPlayer_SubReac (Variables|Default|GetProto%20Game%20Instance)) (Utilities|Array|Get(acopy) (Variables|計算用|GetFormerStatus) 2)))

(fn FBuffVolumeSet
  (params (Buff_Level :type Integer))
  (bind _lostseveritydamage (CallFunction|FSetLostSeverityDamage))
  (LocalVariables|SetLostSeverityDamage _lostseveritydamage)
  (switch int Buff_Level ; 体力回復がどこまでいったかで分岐する\n1：50％以上\n2：75％以上\n3：90％以上\n4：完全回復
    (:1
      (Variables|バフ・デバフ|SetBuff_Volume (Utilities|Select :Index (LocalVariables|GetLostSeverityDamage) :NewEnumerator0 1.0 :NewEnumerator1 1.05 :NewEnumerator2 1.1 :NewEnumerator3 1.2 :NewEnumerator4 1.25))
      (CallFunction|FBuffALLapply :!label _label)
      (Default|StatusLimitCheck (Variables|Default|GetProto%20Game%20Instance)))
    (:2
      (Variables|バフ・デバフ|SetBuff_Volume (Utilities|Select :Index (LocalVariables|GetLostSeverityDamage) :NewEnumerator0 1.0 :NewEnumerator1 1.1 :NewEnumerator2 1.15 :NewEnumerator3 1.25 :NewEnumerator4 1.3))
      (goto _label))
    (:3
      (Variables|バフ・デバフ|SetBuff_Volume (Utilities|Select :Index (LocalVariables|GetLostSeverityDamage) :NewEnumerator0 1.0 :NewEnumerator1 1.15 :NewEnumerator2 1.2 :NewEnumerator3 1.3 :NewEnumerator4 1.4))
      (goto _label))
    (:4
      (Variables|バフ・デバフ|SetBuff_Volume (Utilities|Select :Index (LocalVariables|GetLostSeverityDamage) :NewEnumerator0 1.0 :NewEnumerator1 1.2 :NewEnumerator2 1.3 :NewEnumerator3 1.4 :NewEnumerator4 1.5))
      (CallFunction|FBuffALLapply)
      (CallFunction|FBuffbyBulletStock)
      (Default|StatusLimitCheck (Variables|Default|GetProto%20Game%20Instance)))))

(fn FBuffbyBulletStock
  (bind _proto_game_instance (Variables|Default|GetProto%20Game%20Instance))
  (bind _proto_game_instance_2 (Variables|Default|GetProto%20Game%20Instance))
  (bind _proto_game_instance_3 (Variables|Default|GetProto%20Game%20Instance))
  (Variables|/Game/Data/GI_PlayerStatus.GI_PlayerStatus_C|SetPlayer_ATK _proto_game_instance (+ (Variables|/Game/Data/GI_PlayerStatus.GI_PlayerStatus_C|GetPlayer_ATK _proto_game_instance) (* (Utilities|Array|Get(acopy) (Variables|計算用|GetFormerStatus)) (* (Math|Conversions|ToFloat(Integer) (+ (Variables|計算用|GetRedBulletStock) (Variables|計算用|GetSpecialAttackStock))) 0.01))))
  (Variables|/Game/Data/GI_PlayerStatus.GI_PlayerStatus_C|SetPlayer_SPD _proto_game_instance_3 (+ (Variables|/Game/Data/GI_PlayerStatus.GI_PlayerStatus_C|GetPlayer_SPD _proto_game_instance_3) (* (Utilities|Array|Get(acopy) (Variables|計算用|GetFormerStatus) 1) (* (Math|Conversions|ToFloat(Integer) (+ (Variables|計算用|GetBlueBulletStock) (Variables|計算用|GetSpecialAttackStock))) 0.01))))
  (Variables|/Game/Data/GI_PlayerStatus.GI_PlayerStatus_C|SetPlayer_SubReac _proto_game_instance_2 (- (Variables|/Game/Data/GI_PlayerStatus.GI_PlayerStatus_C|GetPlayer_SubReac _proto_game_instance_2) (* (Utilities|Array|Get(acopy) (Variables|計算用|GetFormerStatus) 2) (* (Math|Conversions|ToFloat(Integer) (+ (Variables|計算用|GetGreenBulletStock) (Variables|計算用|GetSpecialAttackStock))) 0.01))))
  (Variables|計算用|SetRedBulletStock 0)
  (Variables|計算用|SetBlueBulletStock 0)
  (Variables|計算用|SetGreenBulletStock 0)
  (Variables|計算用|SetSpecialAttackStock 0))

(fn FSetLostSeverityDamage
  (bind _proto_game_instance (Variables|Default|GetProto%20Game%20Instance))
  (bind _player_hp (Variables|/Game/Data/GI_PlayerStatus.GI_PlayerStatus_C|GetPlayer_HP _proto_game_instance))
  (if (<= (- 1e+02 (Variables|計算用|GetLostHP)) (* _player_hp 0.1))
    (return "NewEnumerator4")
    (elif (<= (- 1e+02 (Variables|計算用|GetLostHP)) (* _player_hp 0.25))
      (return "NewEnumerator3")
      (elif (<= (- 1e+02 (Variables|計算用|GetLostHP)) (* _player_hp 0.5))
        (return "NewEnumerator2")
        (elif (<= (- 1e+02 (Variables|計算用|GetLostHP)) (* _player_hp 0.75))
          (return "NewEnumerator1")
          (else
            (return "NewEnumerator0")))))))

(fn FMoveCal
  (params (InputVolume :type Float%20%28double-precision%29))
  (bind _proto_game_instance (Variables|Default|GetProto%20Game%20Instance))
  (bind _player_spd (Variables|/Game/Data/GI_PlayerStatus.GI_PlayerStatus_C|GetPlayer_SPD _proto_game_instance))
  (return (* InputVolume (- (* _player_spd (Variables|バフ・デバフ|GetItemSpeedBuff_Volume)) (* _player_spd (Variables|バフ・デバフ|GetDebuff_Volume))))))