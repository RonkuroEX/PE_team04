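; Prototype player special attack (bomb) that repeatedly damages overlapping enemies and enemy bullets for a few seconds, then destroys itself.
; After short delays it plays a fire sound, enables its box collision and starts a looping timer.
; The loop event toggles collision and nudges the actor back and forth to re-trigger overlaps.
; Overlaps on tagged actors spawn hit effects and apply damage, computed at construction from base damage times player attack.
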(event OnComponentBeginOverlap(Box)
  (params (OverlappedComponent :type Primitive%20Component%20Object%20Reference) (OtherActor :type Actor%20Object%20Reference) (OtherComp :type Primitive%20Component%20Object%20Reference) (OtherBodyIndex :type Integer) (bFromSweep :type Boolean) (SweepResult :type Hit%20Result%20Structure%20%28by%20ref%29))
  (if (or (Actor|ActorHasTag OtherActor "Enemy") (Actor|ActorHasTag OtherActor "EnemyBullet"))
    ;[1 1 1] 重くなかったらエフェクトつける
    (Effects|SpawnEmitteratLocation "/Game/FXVarietyPack/Particles/P_ky_hit2.P_ky_hit2" (Transformation|GetActorLocation OtherActor))
    (Game|Damage|ApplyDamage OtherActor (Variables|Default|GetBomDanage) 0 0 "/Script/Engine.DamageType")))

(event Custom|SPAttackLoop
  (bind _box (Variables|Default|GetBox))
  (Collision|SetCollisionEnabled _box "NoCollision")
  (Collision|SetCollisionEnabled _box "QueryOnly")
  (Transformation|SetActorLocation (+ (Transformation|GetActorLocation) "0.010000,0.000000,0.000000") false false)
  (Transformation|SetActorLocation (+ (Transformation|GetActorLocation) "-0.010000,0.000000,0.000000") false false))

(event EventBeginPlay
  (Utilities|FlowControl|Delay 0.5)
  (Audio|PlaySoundatLocation "/Game/Sound/SE/Base/13_Fire.13_Fire" "0, 0, 0" "0, 0, 0" 1.0 1.0 0.0 0 0 0 0)
  (Utilities|FlowControl|Delay 0.5)
  (Collision|SetCollisionEnabled (Variables|Default|GetBox) "QueryAndPhysics")
  (bind _returnvalue (Utilities|Time|SetTimerbyEvent (EventDispatchers|CreateEvent :!event Custom|SPAttackLoop) 0.1 true))
  (Variables|Default|SetSpAttackTimer _returnvalue)
  (Utilities|FlowControl|Delay 5.0)
  (Actor|DestroyActor))

(fn ConstructionScript
  (Variables|Default|SetBomDanage (* (Variables|Default|GetBaseDamage) (Variables|Default|GetPlayerATK))) ; ベースダメージ×プレイヤーの攻撃力が最終的なボムのダメージになります
)