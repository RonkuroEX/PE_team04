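; PC_Shooting is the shooting player controller Blueprint that switches Enhanced Input mapping contexts between gameplay, menu and tutorial.
; Two IFF events remove the player context, wait one tick, then add either the menu or the tutorial context.
; The undo event removes both menu and tutorial contexts and immediately restores the player context.
; All changes go through the local player subsystem of player controller 0.
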(event EventIFFChangeIAC
  (bind _returnvalue (Game|GetPlayerController 0))
  (bind _returnvalue_2 (PlayerController|LocalPlayerSubsystems|GetEnhancedInputLocalPlayerSubsystem _returnvalue))
  (Input|RemoveMappingContext _returnvalue_2 "/Game/Input/Shooting/IAC_Player.IAC_Player" "(bIgnoreAllPressedKeysUntilRelease=True,bForceImmediately=False,bNotifyUserSettings=False)")
  (Utilities|FlowControl|DelayUntilNextTick)
  (Input|AddMappingContext _returnvalue_2 "/Game/Input/Menu/IAC_Menu.IAC_Menu" 0 "(bIgnoreAllPressedKeysUntilRelease=True,bForceImmediately=False,bNotifyUserSettings=False)"))

(event EventIFFUndoIAC
  (bind _returnvalue (Game|GetPlayerController 0))
  (bind _returnvalue_2 (PlayerController|LocalPlayerSubsystems|GetEnhancedInputLocalPlayerSubsystem _returnvalue))
  (Input|RemoveMappingContext _returnvalue_2 "/Game/Input/Menu/IAC_Menu.IAC_Menu" "(bIgnoreAllPressedKeysUntilRelease=True,bForceImmediately=False,bNotifyUserSettings=False)")
  (Input|RemoveMappingContext _returnvalue_2 "/Game/Input/Tutorial/IAC_Tutorial.IAC_Tutorial" "(bIgnoreAllPressedKeysUntilRelease=True,bForceImmediately=False,bNotifyUserSettings=False)")
  (Input|AddMappingContext _returnvalue_2 "/Game/Input/Shooting/IAC_Player.IAC_Player" 0 "(bIgnoreAllPressedKeysUntilRelease=True,bForceImmediately=False,bNotifyUserSettings=False)"))

(event EventIFFChangeIACT
  (bind _returnvalue (Game|GetPlayerController 0))
  (bind _returnvalue_2 (PlayerController|LocalPlayerSubsystems|GetEnhancedInputLocalPlayerSubsystem _returnvalue))
  (Input|RemoveMappingContext _returnvalue_2 "/Game/Input/Shooting/IAC_Player.IAC_Player" "(bIgnoreAllPressedKeysUntilRelease=True,bForceImmediately=False,bNotifyUserSettings=False)")
  (Utilities|FlowControl|DelayUntilNextTick)
  (Input|AddMappingContext _returnvalue_2 "/Game/Input/Tutorial/IAC_Tutorial.IAC_Tutorial" 0 "(bIgnoreAllPressedKeysUntilRelease=True,bForceImmediately=False,bNotifyUserSettings=False)"))

(fn ConstructionScript)