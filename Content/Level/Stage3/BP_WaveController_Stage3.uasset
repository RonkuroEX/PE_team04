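; Wave controller for Stage 3 that paces enemy waves and boss fights by streaming sublevels in and out, with names built from a stage prefix.
; An enemy countdown unloads each cleared wave and loads the next, switching to the mini-boss after wave 5 and the stage boss after wave 8.
; Mini-boss unload sets off a flag call and resumes waves; the GameMode receives the stage boss warning and delayed stage-clear messages.
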(event EventBeginPlay
  ;[1 1 1] Waveロードの開始
  (Utilities|FlowControl|Delay 6.0)
  (CallFunction|IFFWaveLoad))

(event EventIFFBossWaveUnLoad
  (params (FromStageBoss :type Boolean))
  ;[1 1 1] ボスWaveサブレベルのアンロード
  (if FromStageBoss
    (Game|UnloadStreamLevel(byName) (Utilities|String|StringToName (Utilities|String|Append (Variables|Default|GetStageNameTemp) "StageBoss")) false)
    (Utilities|FlowControl|Delay 18.0)
    (Class|IFGamemode|IFFStageClear(Message) (Game|GetGameMode))
    (else
      (Game|UnloadStreamLevel(byName) (Utilities|String|StringToName (Utilities|String|Append (Variables|Default|GetStageNameTemp) "MiniBoss")) false)
      (CallFunction|AfterMiniBossFlag)
      (CallFunction|IFFWaveLoad))))

(event EventIFFSetEnemyCount
  (params (EnemyCount :type Integer) (plus1 :type Boolean))
  ;[1 1 1] Wave毎の敵総数のセット＆敵残数の確認（残数0で次のWaveへ移動）
  (Variables|Default|SetWaveEnemyCount EnemyCount))

(event EventIFFDecreaseEnemyCount
  ;[1 1 1] Wave毎の敵総数のセット＆敵残数の確認（残数0で次のWaveへ移動）
  (bind _result (Math|Integer|DecrementInt (Variables|Default|GetWaveEnemyCount))
    (:%20%20
      (if (<= _result 0)
        (CallFunction|IFFWaveUnLoad)
        (switch string (Utilities|String|ToString(Integer) (Variables|Default|GetWaveCount))
          (:Default
            (CallFunction|IFFWaveLoad))
          (:5
            (CallFunction|IFFBossWaveLoad false))
          (:8
            (CallFunction|IFFBossWaveLoad true)))
        (else
          (Development|PrintString (Utilities|String|ToString(Integer) (Variables|Default|GetWaveEnemyCount))))))))

(event EventIFFWaveUnLoad
  ;[1 1 1] Waveサブレベルのアンロード
  (Game|UnloadStreamLevel(byName) (Utilities|String|StringToName (Utilities|String|Append (Variables|Default|GetStageNameTemp) "Wave" (Utilities|String|ToString(Integer) (Variables|Default|GetWaveCount)))) false))

(event EventIFFWaveLoad
  ;[1 1 1] Waveサブレベルのロード
  (Math|Integer|IncrementInt (Variables|Default|GetWaveCount)
    (:%20%20
      (Game|LoadStreamLevel(byName) (Utilities|String|StringToName (Utilities|String|Append (Variables|Default|GetStageNameTemp) "Wave" (Utilities|String|ToString(Integer) (Variables|Default|GetWaveCount)))) true true))))

(event EventIFFBossWaveLoad
  (params (ForStageBoss :type Boolean))
  ;[1 1 1] ボスWaveサブレベルのロード
  (if ForStageBoss
    (Class|IFGamemode|IFFWarning(Message) (Game|GetGameMode))
    (Utilities|FlowControl|Delay 6.0)
    (Game|LoadStreamLevel(byName) (Utilities|String|StringToName (Utilities|String|Append (Variables|Default|GetStageNameTemp) "StageBoss")) true true)
    (else
      (Utilities|FlowControl|Delay 3.0)
      (Game|LoadStreamLevel(byName) (Utilities|String|StringToName (Utilities|String|Append (Variables|Default|GetStageNameTemp) "MiniBoss")) true true))))

(fn ConstructionScript
  (|CallParentFunction))