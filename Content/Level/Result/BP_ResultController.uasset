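; Result screen controller that creates WBP_Result on BeginPlay and animates the player's scores counting up.
; It reads heal, kill and bomb scores from the GI_PlayerStatus game instance.
; Timelines lerp each value from zero in sequence (heal, kill, bomb, then their summed total), with one-second delays between steps.
; When the total finishes, it passes the truncated total to the widget's ClearRankJudge to determine the clear rank.
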(event Custom|LerpBombScore
  ;[1 1 1] リザルトＵＩに各スコアの数値をカウントアップ式で渡す
  (bind _lerpflow (Timeline|LerpBombScoreTimeline Play)
    (:Update
      (Default|UpdateBombScore (Variables|Default|GetResultUI) (Math|Float|Truncate (Math|Float|Lerp 0.0 (Variables|/Game/Data/GI_PlayerStatus.GI_PlayerStatus_C|GetBombScore (Variables|Default|GetGI%20Player%20Status)) _lerpflow))))
    (:Finished
      (Utilities|FlowControl|Delay 1.0)
      (CallFunction|LerpTotalScore))))

(event Custom|LerpHealScore
  ;[1 1 1] リザルトＵＩに各スコアの数値をカウントアップ式で渡す
  (bind _lerpflow (Timeline|LerpHealScoreTimeline Play)
    (:Update
      (Default|UpdateHealScore (Variables|Default|GetResultUI) (Math|Float|Truncate (Math|Float|Lerp 0.0 (Variables|/Game/Data/GI_PlayerStatus.GI_PlayerStatus_C|GetHealScore (Variables|Default|GetGI%20Player%20Status)) _lerpflow))))
    (:Finished
      (Utilities|FlowControl|Delay 1.0)
      (CallFunction|LerpKillScore))))

(event Custom|LerpKillScore
  ;[1 1 1] リザルトＵＩに各スコアの数値をカウントアップ式で渡す
  (bind _lerpflow (Timeline|LerpKillScoreTimeline Play)
    (:Update
      (Default|UpdateKillScore (Variables|Default|GetResultUI) (Math|Float|Truncate (Math|Float|Lerp 0.0 (Variables|/Game/Data/GI_PlayerStatus.GI_PlayerStatus_C|GetKillScore (Variables|Default|GetGI%20Player%20Status)) _lerpflow))))
    (:Finished
      (Utilities|FlowControl|Delay 1.0)
      (CallFunction|LerpBombScore))))

(event Custom|LerpTotalScore
  (bind _gi_player_status (Variables|Default|GetGI%20Player%20Status))
  ;[1 1 1] リザルトＵＩに総スコアの数値をカウントアップ式で渡す→クリアランク表示のイベントを呼び出す
  (Variables|Default|SetTotalScore (+ (Variables|/Game/Data/GI_PlayerStatus.GI_PlayerStatus_C|GetHealScore _gi_player_status) (Variables|/Game/Data/GI_PlayerStatus.GI_PlayerStatus_C|GetKillScore _gi_player_status) (Variables|/Game/Data/GI_PlayerStatus.GI_PlayerStatus_C|GetBombScore _gi_player_status)))
  (bind _lerpflow (Timeline|タイムライン Play)
    (:Update
      (Default|UpdateTotalScore (Variables|Default|GetResultUI) (Math|Float|Truncate (Math|Float|Lerp 0.0 (Variables|Default|GetTotalScore) _lerpflow))))
    (:Finished
      (Default|ClearRankJudge (Variables|Default|GetResultUI) (Math|Float|Truncate (Variables|Default|GetTotalScore))))))

(event EventBeginPlay
  (bind _returnvalue (UserInterface|CreateWidget "/Game/UI/Result/WBP_Result.WBP_Result_C"))
  (bind _output_get (Variables|Default|SetResultUI _returnvalue))
  (UserInterface|Viewport|AddtoViewport _output_get 0)
  (bind _asgi_player_status (Utilities|Casting|CastToGI_PlayerStatus (Game|GetGameInstance)))
  (Variables|Default|SetGI%20Player%20Status _asgi_player_status)
  (Utilities|FlowControl|Delay 1.0)
  (CallFunction|LerpHealScore))

(fn ConstructionScript)