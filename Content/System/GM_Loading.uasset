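; GM_Loading, apparently the game mode for a loading level, shows a loading screen and then travels to the requested stage or title level.
; On BeginPlay it opens the loading media, adds WBP_Loading to the viewport and maps the game instance's stage message to a level name.
; It starts a hidden, non-blocking stream load of that level, then opens it by name after a fixed delay without checking load completion.
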(event EventBeginPlay
  (Media|MediaPlayer|OpenSource (Variables|Default|GetMadiaPlayer) "/Game/Movies/loading.loading")
  (bind _returnvalue (UserInterface|CreateWidget "/Game/UI/Loading/WBP_Loading.WBP_Loading_C"))
  (bind _output_get (Variables|Default|SetLoadingScreen _returnvalue))
  (UserInterface|Viewport|AddtoViewport _output_get 0)
  (bind _stagelevel (Class|IFPlayerStatus|IFFGetStageLevel(Message) (Game|GetGameInstance)))
  (switch Utilities|FlowControl|Switch|SwitchonE_StageLevel _stagelevel
    (:NewEnumerator0
      (Variables|Default|SetLevel%20Name "L_Stage1"))
    (:NewEnumerator1
      (Variables|Default|SetLevel%20Name "L_Stage2"))
    (:NewEnumerator2
      (Variables|Default|SetLevel%20Name "L_Stage3"))
    (:NewEnumerator3
      (Variables|Default|SetLevel%20Name "L_Title")))
  (Game|LoadStreamLevel(byName) (Variables|Default|GetLevel%20Name) false)
  (Utilities|FlowControl|Delay 2.0)
  (Game|OpenLevel(byName) (Variables|Default|GetLevel%20Name)))

(fn ConstructionScript)