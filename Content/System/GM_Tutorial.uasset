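; Tutorial game mode that runs a play session's HUD, background music and player sound effects.
; BeginPlay creates the WBP_PlayMaster HUD, starts the BGM and adds input mappings after a delay.
; Interface events relay items, damage, warnings, boss HP, game over and clear to the HUD and audio, including boss BGM fades.
; The construction script sets the GameInstance stage from the level name (marked debug-only), then blocking-loads that stage's sounds from data assets.
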(event EventBeginPlay
  (bind _returnvalue (UserInterface|CreateWidget "/Game/UI/PlayMenu/WBP_PlayMaster.WBP_PlayMaster_C"))
  (bind _output_get (Variables|Default|SetWBP_PlayMaster _returnvalue))
  (UserInterface|Viewport|AddtoViewport _output_get 1)
  (Default|SetItemVisibility (Variables|Default|GetWBP_PlayMaster))
  (Class|IFGamemode|IFFChangeUIWayLavel(Message) (Game|GetGameMode))
  (Audio|Components|Audio|Play (Variables|コンポーネント|GetAC_PlayBGM) 0.0)
  (Utilities|FlowControl|Delay 3.0)
  (Input|AddMappingContext (PlayerController|LocalPlayerSubsystems|GetEnhancedInputLocalPlayerSubsystem (Game|GetPlayerController 0)) "/Game/Input/Shooting/IAC_Player.IAC_Player" 0 "(bIgnoreAllPressedKeysUntilRelease=True,bForceImmediately=False,bNotifyUserSettings=False)")
  (Input|AddMappingContext (PlayerController|LocalPlayerSubsystems|GetEnhancedInputLocalPlayerSubsystem (Game|GetPlayerController 0)) "/Game/Input/Debug/IAC_Debug.IAC_Debug" 0 "(bIgnoreAllPressedKeysUntilRelease=True,bForceImmediately=False,bNotifyUserSettings=False)"))

(event EventIFFGameOver
  (bind _returnvalue (Game|GetPlayerCharacter 0))
  (bind _returnvalue_2 (Transformation|GetActorLocation _returnvalue))
  (Audio|PlaySoundatLocation (Variables|Default|GetDeathSE) _returnvalue_2 "0, 0, 0" 1.0 1.0 0.1 0 0 0 0)
  (Niagara|SpawnSystematLocation (Variables|Default|GetFX_PlayerExplode) _returnvalue_2)
  (Utilities|FlowControl|Delay 1.0)
  (Audio|Components|Audio|Stop (Variables|Default|GetAC_BossBGM))
  (Default|GameOver (Variables|Default|GetWBP_PlayMaster))
  (Audio|Components|Audio|Play (Variables|Default|GetAC_GameOverBGM) 0.0))

(event EventIFFStageClear
  (Default|GameClear (Variables|Default|GetWBP_PlayMaster)))

(event EventIFFPlayerSuperRecover
  (params (StopRecover :type Boolean))
  (if StopRecover
    (Class|AudioComponent|SetPaused (Variables|Default|GetSPRecoverSE) true)
    (else
      (Audio|Components|Audio|Play (Variables|Default|GetSPRecoverSE) 0.0)
      (Class|AudioComponent|SetPaused (Variables|Default|GetSPRecoverSE) false))))

(event EventIFFBossExit
  (Variables|/Script/UMG.Widget|SetVisibility (Variables|/Game/UI/PlayMenu/WBP_PlayMaster.WBP_PlayMaster_C|GetBossHPber (Variables|Default|GetWBP_PlayMaster)) "Hidden"))

(event EventIFFSetBossHP
  (params (CurrentBossHP :type Float%20%28double-precision%29))
  (Variables|/Game/UI/PlayMenu/WBP_PlayMaster.WBP_PlayMaster_C|SetCurrentBossHp (Variables|Default|GetWBP_PlayMaster) CurrentBossHP))

(event EventIFFBossAppearance
  (params (MaxBossHP :type Float%20%28double-precision%29))
  (bind _wbp_playmaster (Variables|Default|GetWBP_PlayMaster))
  (bind _output_get (Variables|/Game/UI/PlayMenu/WBP_PlayMaster.WBP_PlayMaster_C|SetMaxBossHP _wbp_playmaster MaxBossHP))
  (Variables|/Game/UI/PlayMenu/WBP_PlayMaster.WBP_PlayMaster_C|SetCurrentBossHp _wbp_playmaster _output_get)
  (Variables|/Script/UMG.Widget|SetVisibility (Variables|/Game/UI/PlayMenu/WBP_PlayMaster.WBP_PlayMaster_C|GetBossHPber (Variables|Default|GetWBP_PlayMaster)) "HitTestInvisible"))

(event EventIFFWarning
  (bind _wbp_playmaster (Variables|Default|GetWBP_PlayMaster))
  (bind _wbp_warning (Variables|/Game/UI/PlayMenu/WBP_PlayMaster.WBP_PlayMaster_C|GetWBP_Warning _wbp_playmaster))
  (Variables|/Script/UMG.Widget|SetVisibility _wbp_warning "HitTestInvisible")
  (Default|WarningAnim _wbp_warning))

(event EventIFFPlayerDamage
  (Audio|PlaySoundatLocation (Variables|Default|GetDamageSE) (Transformation|GetActorLocation (Game|GetPlayerCharacter 0)) "0, 0, 0" 1.0 1.0 0.0 0 0 0 0)
  (CallFunction|IFFPlayerSuperRecover true))

(event EventIFFChangeUIWayLavel
  (Default|ChangeWayLevel (Variables|Default|GetWBP_PlayMaster)))

(event EventIFFItem
  (params (ItemType :type E_ItemType%20Enum :default "NewEnumerator0") (ItemTime :type Float%20%28double-precision%29))
  (bind _wbp_playmaster (Variables|Default|GetWBP_PlayMaster))
  (switch Utilities|FlowControl|Switch|SwitchonE_ItemType ItemType
    (:NewEnumerator0
      (Default|ItemATKTimerSet _wbp_playmaster ItemTime))
    (:NewEnumerator1
      (Default|ItemSPDTimerSet _wbp_playmaster ItemTime))
    (:NewEnumerator2
      (Default|ItemRECTimerSet _wbp_playmaster ItemTime))
    (:NewEnumerator3
      (Default|SetItemVisibility _wbp_playmaster)))
  (if (> ItemTime 0.0)
    (Audio|PlaySoundatLocation (Variables|Default|GetGetItemSE) (Transformation|GetActorLocation (Game|GetPlayerCharacter 0)) "0, 0, 0" 1.0 1.0 0.0 0 0 0 0)))

(event EventIFFPlayBossBGM
  (Audio|Components|Audio|FadeOut (Variables|コンポーネント|GetAC_PlayBGM) 1.0 0.0 "Linear" :!class /Script/Engine.AudioComponent)
  (Audio|Components|Audio|Play (Variables|Default|GetAC_BossBGM) 0.0))

(event EventIFFStopBossBGM
  (Audio|Components|Audio|FadeOut (Variables|Default|GetAC_BossBGM) 1.0 0.0 "Linear" :!class /Script/Engine.AudioComponent)
  (Audio|Components|Audio|FadeIn (Variables|コンポーネント|GetAC_PlayBGM) 1.0 1.0 0.0 "Linear" :!class /Script/Engine.AudioComponent))

(fn ConstructionScript
  (bind _returnvalue (Game|GetGameInstance))
  (bind _returnvalue_2 (Game|GetCurrentLevelName true))
  ;[1 1 1] デバッグ用にのみ必要な処理
  (switch string _returnvalue_2
    (:L_Stage1
      (Class|IFPlayerStatus|IFFSetStage(Message) _returnvalue "NewEnumerator0"))
    (:L_Stage2
      (Class|IFPlayerStatus|IFFSetStage(Message) _returnvalue "NewEnumerator1"))
    (:L_Stage3
      (Class|IFPlayerStatus|IFFSetStage(Message) _returnvalue "NewEnumerator2"))
    (:L_Tutorial
      (Class|IFPlayerStatus|IFFSetStage(Message) _returnvalue "NewEnumerator4")))
  (CallFunction|FSetBGM)
  (CallFunction|FSetPlayerSE)
  (Class|IFPlayerStatus|IFFSaveStatus(Message) (Game|GetGameInstance)))

(fn FSetBGM
  (bind _da_playbgm (Variables|BGM|GetDA_PlayBGM))
  (bind _da_playbgm_2 (Variables|BGM|GetDA_PlayBGM))
  (bind _stagelevel (Class|IFPlayerStatus|IFFGetStageLevel(Message) (Game|GetGameInstance)))
  (switch Utilities|FlowControl|Switch|SwitchonE_StageLevel _stagelevel
    (:NewEnumerator0
      (bind _returnvalue (Utilities|LoadAssetBlocking (Variables|/Game/Sound/DataAsset/Template/DA_PlayBGMTemp.DA_PlayBGMTemp_C|GetStage1BGM _da_playbgm_2)))
      (bind _returnvalue_2 (Utilities|LoadAssetBlocking (Variables|/Game/Sound/DataAsset/Template/DA_PlayBGMTemp.DA_PlayBGMTemp_C|GetStage1BossBGM _da_playbgm_2)))
      (CallFunction|FCastandSetBGM _returnvalue _returnvalue_2))
    (:NewEnumerator1
      (bind _returnvalue_3 (Utilities|LoadAssetBlocking (Variables|/Game/Sound/DataAsset/Template/DA_PlayBGMTemp.DA_PlayBGMTemp_C|GetStage2BGM _da_playbgm_2)))
      (bind _returnvalue_4 (Utilities|LoadAssetBlocking (Variables|/Game/Sound/DataAsset/Template/DA_PlayBGMTemp.DA_PlayBGMTemp_C|GetStage2BossBGM _da_playbgm_2)))
      (CallFunction|FCastandSetBGM _returnvalue_3 _returnvalue_4))
    (:NewEnumerator2
      (bind _returnvalue_5 (Utilities|LoadAssetBlocking (Variables|/Game/Sound/DataAsset/Template/DA_PlayBGMTemp.DA_PlayBGMTemp_C|GetStage3BGM _da_playbgm_2)))
      (bind _returnvalue_6 (Utilities|LoadAssetBlocking (Variables|/Game/Sound/DataAsset/Template/DA_PlayBGMTemp.DA_PlayBGMTemp_C|GetStage3BossBGM _da_playbgm_2)))
      (CallFunction|FCastandSetBGM _returnvalue_5 _returnvalue_6))
    (:NewEnumerator4
      (bind _returnvalue_7 (Utilities|LoadAssetBlocking (Variables|/Game/Sound/DataAsset/Template/DA_PlayBGMTemp.DA_PlayBGMTemp_C|GetStage1BGM _da_playbgm_2)))
      (bind _returnvalue_8 (Utilities|LoadAssetBlocking (Variables|/Game/Sound/DataAsset/Template/DA_PlayBGMTemp.DA_PlayBGMTemp_C|GetStage1BossBGM _da_playbgm_2)))
      (CallFunction|FCastandSetBGM _returnvalue_7 _returnvalue_8)))
  (Utilities|FlowControl|Sequence
    (:then_0
      (bind _returnvalue_9 (Utilities|LoadAssetBlocking (Variables|/Game/Sound/DataAsset/Template/DA_PlayBGMTemp.DA_PlayBGMTemp_C|GetGameOverBGM _da_playbgm)))
      (bind _assound_cue (Utilities|Casting|CastToSoundCue _returnvalue_9))
      (bind _returnvalue_10 (Audio|CreateSound2D _assound_cue 1.0 1.0 0.0 0 false false))
      (Variables|Default|SetAC_GameOverBGM _returnvalue_10))
    (:then_1
      (bind _returnvalue_11 (Utilities|LoadAssetBlocking (Variables|/Game/Sound/DataAsset/Template/DA_PlayBGMTemp.DA_PlayBGMTemp_C|GetGameClearBGM _da_playbgm)))
      (bind _assound_cue_2 (Utilities|Casting|CastToSoundCue _returnvalue_11))
      (bind _returnvalue_12 (Audio|CreateSound2D _assound_cue_2 1.0 1.0 0.0 0 false false))
      (Variables|Default|SetAC_GameClearBGM _returnvalue_12))))

(fn FSetPlayerSE
  (bind _da_playerse (Variables|Default|GetDA_PlayerSE))
  (Utilities|FlowControl|Sequence
    (:then_0
      (bind _returnvalue (Utilities|LoadAssetBlocking (Variables|/Game/Sound/DataAsset/Template/DA_PlayerSETemp.DA_PlayerSETemp_C|GetGetItemSE _da_playerse)))
      (bind _assound_cue (Utilities|Casting|CastToSoundCue _returnvalue))
      (Variables|Default|SetGetItemSE _assound_cue))
    (:then_1
      (bind _returnvalue_2 (Utilities|LoadAssetBlocking (Variables|/Game/Sound/DataAsset/Template/DA_PlayerSETemp.DA_PlayerSETemp_C|GetDeathSE _da_playerse)))
      (bind _assound_cue_2 (Utilities|Casting|CastToSoundCue _returnvalue_2))
      (Variables|Default|SetDeathSE _assound_cue_2))
    (:then_2
      (bind _returnvalue_3 (Utilities|LoadAssetBlocking (Variables|/Game/Sound/DataAsset/Template/DA_PlayerSETemp.DA_PlayerSETemp_C|GetSuperRecoverSE _da_playerse)))
      (bind _assound_cue_3 (Utilities|Casting|CastToSoundCue _returnvalue_3))
      (bind _returnvalue_4 (Audio|CreateSound2D _assound_cue_3 1.0 1.0 0.0 0))
      (Variables|Default|SetSPRecoverSE _returnvalue_4))
    (:then_3
      (bind _returnvalue_5 (Utilities|LoadAssetBlocking (Variables|/Game/Sound/DataAsset/Template/DA_PlayerSETemp.DA_PlayerSETemp_C|GetDamageSE _da_playerse)))
      (bind _assound_cue_4 (Utilities|Casting|CastToSoundCue _returnvalue_5))
      (Variables|Default|SetDamageSE _assound_cue_4))))

(fn FCastandSetBGM
  (params (BGM :type Object%20Object%20Reference) (BossBGM :type Object%20Object%20Reference))
  (Utilities|FlowControl|Sequence
    (:then_0
      (bind _assound_cue (Utilities|Casting|CastToSoundCue BGM))
      (bind _returnvalue (Audio|CreateSound2D _assound_cue 1.0 1.0 0.0 0 false false))
      (Variables|コンポーネント|SetAC_PlayBGM _returnvalue))
    (:then_1
      (bind _assound_cue_2 (Utilities|Casting|CastToSoundCue BossBGM))
      (bind _returnvalue_2 (Audio|CreateSound2D _assound_cue_2 1.0 1.0 0.0 0 false false))
      (Variables|Default|SetAC_BossBGM _returnvalue_2))))