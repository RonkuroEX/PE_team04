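; GM_Title is the title screen game mode that sets up menu input and starts the background music.
; BeginPlay adds the IAC_Menu mapping context, then creates a 2D audio component from the loaded BGM, keeps it and plays it.
; F_SetBGM synchronously loads the SoundCue from a soft reference in the DATitleBGM data asset.
; The construction script pushes the SCM_Master sound mix.
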(event EventBeginPlay
  (Input|AddMappingContext (PlayerController|LocalPlayerSubsystems|GetEnhancedInputLocalPlayerSubsystem (Game|GetPlayerController 0)) "/Game/Input/Menu/IAC_Menu.IAC_Menu" 0 "(bIgnoreAllPressedKeysUntilRelease=True,bForceImmediately=False,bNotifyUserSettings=False)")
  (bind _assound_cue (CallFunction|FSetBGM)) ; データアセットのソフト参照を元にBGMをロード
  (bind _returnvalue (Audio|CreateSound2D _assound_cue 1.0 1.0 0.0 0))
  (bind _output_get (Variables|Default|SetAC_TitleBGM _returnvalue))
  (Audio|Components|Audio|Play _output_get 0.0))

(fn ConstructionScript
  (Audio|PushSoundMixModifier "/Game/Sound/SCM_Master.SCM_Master"))

(fn FSetBGM
  (bind _returnvalue (Utilities|LoadAssetBlocking (Variables|/Game/System/DataAsset/Template/DA_TitleBGMTemp.DA_TitleBGMTemp_C|GetTitleBGM (Variables|Default|GetDA_TitleBGM))))
  (bind _assound_cue (Utilities|Casting|CastToSoundCue _returnvalue))
  (return _assound_cue))