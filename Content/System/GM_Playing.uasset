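; GM_Playing appears to be the gameplay game mode, setting up player input and relaying game events to the main play HUD.
; On BeginPlay it adds the IAC_Player Enhanced Input mapping context, creates WBP_PlayMaster and refreshes its item visibility.
; IFF events forward game over and item pickups to that widget by item type: attack, speed and recovery set timers, while SP attack count refreshes visibility.
; The move speed timer receives zero instead of the passed item time.
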(event EventBeginPlay
  (Input|AddMappingContext (PlayerController|LocalPlayerSubsystems|GetEnhancedInputLocalPlayerSubsystem (Game|GetPlayerController 0)) "/Game/Input/Shooting/IAC_Player.IAC_Player" 0 "(bIgnoreAllPressedKeysUntilRelease=True,bForceImmediately=False,bNotifyUserSettings=False)")
  (bind _returnvalue (UserInterface|CreateWidget "/Game/UI/PlayMenu/WBP_PlayMaster.WBP_PlayMaster_C"))
  (bind _output_get (Variables|Default|SetWBP_PlayMaster _returnvalue))
  (UserInterface|Viewport|AddtoViewport _output_get 0)
  (Default|SetItemVisibility (Variables|Default|GetWBP_PlayMaster)))

(event EventIFFGameOver
  (Default|GameOver (Variables|Default|GetWBP_PlayMaster)))

(event EventIFFItem
  (params (ItemType :type E_ItemType%20Enum :default "NewEnumerator0") (ItemTime :type Float%20%28double-precision%29))
  (bind _wbp_playmaster (Variables|Default|GetWBP_PlayMaster))
  (switch Utilities|FlowControl|Switch|SwitchonE_ItemType ItemType
    (:NewEnumerator0
      (Default|ItemATKTimerSet _wbp_playmaster ItemTime))
    (:NewEnumerator1
      (Default|ItemSPDTimerSet _wbp_playmaster 0.0))
    (:NewEnumerator2
      (Default|ItemRECTimerSet _wbp_playmaster ItemTime))
    (:NewEnumerator3
      (Default|SetItemVisibility _wbp_playmaster))))

(fn ConstructionScript)