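; BP_ProtoItem is a prototype pickup item that applies its effect when the player touches it.
; A Sphere overlap with the player pawn sends the item's type through the IFFItemAdhibitionMessage interface call, then destroys the actor.
; Tick spins the item around its yaw axis by a fixed step each frame, independent of delta time.
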(event OnComponentBeginOverlap(Sphere)
  (params (OverlappedComponent :type Primitive%20Component%20Object%20Reference) (OtherActor :type Actor%20Object%20Reference) (OtherComp :type Primitive%20Component%20Object%20Reference) (OtherBodyIndex :type Integer) (bFromSweep :type Boolean) (SweepResult :type Hit%20Result%20Structure%20%28by%20ref%29))
  ;[1 1 1] プレイヤーが接触した際のアイテム効果適用
  (if (== OtherActor (Game|Player|GetPlayerPawn 0))
    (Class|IFPlayer|IFFItemAdhibition(Message) (Game|Player|GetPlayerPawn 0) (Variables|Default|GetItemType))
    (Actor|DestroyActor)))

(event EventTick
  (params (DeltaSeconds :type Float%20%28single-precision%29))
  (bind _returnvalue (Transformation|GetActorRotation))
  (Transformation|SetActorRotation (Math|Rotator|MakeRotator (.roll _returnvalue) (.pitch _returnvalue) (+ (.yaw _returnvalue) 5.0))))

(fn ConstructionScript)