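; Prototype enemy base that travels along a target spline while facing the player, then destroys itself at the end.
; A timeline scaled by TimeLength drives spline distance, with EEnemyMoveType selecting a constant or pause-at-half curve.
; When damage depletes HP, weighted random draws from two DataTables pick drop count and each item type, spawning BP_ProtoItem before destruction.
; SpawnBullet is an empty event.
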(event Custom|SpawnBullet)

(event EventBeginPlay
  (bind _targetspline (Variables|Default|GetTargetSpline))
  (bind _asgi_player_status (Utilities|Casting|CastToGI_PlayerStatus (Game|GetGameInstance)))
  (Variables|Default|SetAs%20GI%20Player%20Status _asgi_player_status)
  (Components|Timeline|SetPlayRate (Variables|Default|GetTimeline_Spline) (/ 1.0 (Variables|Default|GetTimeLength)))
  (bind (_direction _constant _pauseathalf) (Timeline|Timeline_Spline Play)
    (:Update
      (switch Utilities|FlowControl|Switch|SwitchonE_EnemyMoveType (Variables|Default|GetE_EnemyMoveType)
        (:NewEnumerator0
          (Variables|Default|SetTimelineValue _constant))
        (:NewEnumerator1
          (Variables|Default|SetTimelineValue _pauseathalf)))
      (Transformation|SetActorTransform (Math|Transform|MakeTransform (Spline|GetLocationatDistanceAlongSpline _targetspline (* (Variables|Default|GetTimelineValue) (Spline|GetSplineLength _targetspline)) "World") (Math|Rotator|FindLookatRotation (Transformation|GetWorldLocation (Variables|Default|GetBox)) (Transformation|GetActorLocation (Game|Player|GetPlayerPawn 0))) "1.000000,1.000000,1.000000")))
    (:Finished
      (Actor|DestroyActor))))

(event Game|Damage|EventAnyDamage
  (params (Damage :type Float%20%28single-precision%29) (DamageType :type Damage%20Type%20Object%20Reference) (InstigatedBy :type Controller%20Object%20Reference) (DamageCauser :type Actor%20Object%20Reference))
  (bind _output_get (Variables|Default|SetHP (- (Variables|Default|GetHP) Damage)))
  (if (not (> _output_get 0.0))
    (bind _dropnum (CallFunction|FChooseDropNum)) ; ドロップするアイテムの数を抽選する
    (if (> _dropnum 0) ; ドロップする数が０より大きいか
      (for _index (range 1 _dropnum) ; ドロップ数分ループを回す
        (Variables|Default|SetTotalRate 0.0) ; ループ前にリセット
        (bind _itemtype (CallFunction|FChooseDropItem)) ; ドロップするアイテムを抽選する
        (bind _returnvalue (Game|SpawnActorfromClass "/Game/proto/BP/Item/BP_ProtoItem.BP_ProtoItem_C" (Math|Transform|MakeTransform (Transformation|GetActorLocation) "0, 0, 0" "1.000000,1.000000,1.000000") "AdjustIfPossibleButAlwaysSpawn" "OverrideRootScale" 0 0)) ; アイテムをドロップする
        (Default|GetItemType _returnvalue _itemtype))
      (Actor|DestroyActor)
      (else
        (Actor|DestroyActor)))))

(fn ConstructionScript)

(fn FChooseDropNum
  (bind _outrownames (DataTable|GetDataTableRowNames (Variables|Default|GetDropNumTable))) ; データテーブルの行名を取得
  (for _array_element _outrownames
    (bind _returnvalue (Utilities|GetDataTableRow (Variables|Default|GetDropNumTable) _array_element) ; 入れられたデータテーブルの指定の行名の情報を取得
      (:then
        (Variables|Default|SetTotalRate (+ (.Rate (Utilities|Struct|BreakS_DropNum _returnvalue)) (Variables|Default|GetTotalRate))) ; 各確率の合計値を出す
      )))
  (Variables|Default|SetRandomPoint (* (Math|Random|RandomFloat) (Variables|Default|GetTotalRate))) ; レート合計値の1倍~0倍の数値を取得する
  (bind _outrownames_2 (DataTable|GetDataTableRowNames (Variables|Default|GetDropNumTable)))
  (for _array_element_2 _outrownames_2
    (bind _returnvalue_2 (Utilities|GetDataTableRow (Variables|Default|GetDropNumTable) _array_element_2)
      (:then
        (if (< (Variables|Default|GetRandomPoint) (.Rate (Utilities|Struct|BreakS_DropNum _returnvalue_2))) ; アイテムレートよりランダムポイントのレートが少ないか
          (return (.Num (Utilities|Struct|BreakS_DropNum _returnvalue_2)))
          (else
            (Variables|Default|SetRandomPoint (- (Variables|Default|GetRandomPoint) (.Rate (Utilities|Struct|BreakS_DropNum _returnvalue_2)))) ; ランダムポイントからそのアイテムのレートを引いて次ループの当選率を上げる
          ))))))

(fn FChooseDropItem
  (bind _outrownames (DataTable|GetDataTableRowNames (Variables|Default|GetDropItemTable))) ; データテーブルの行名を取得
  (for _array_element _outrownames
    (bind _returnvalue (Utilities|GetDataTableRow (Variables|Default|GetDropItemTable) _array_element) ; 入れられたデータテーブルの指定の行名の情報を取得
      (:then
        (Variables|Default|SetTotalRate (+ (.Rate (Utilities|Struct|BreakS_DropItem _returnvalue)) (Variables|Default|GetTotalRate))) ; 各確率の合計値を出す
      )))
  (Variables|Default|SetRandomPoint (* (Math|Random|RandomFloat) (Variables|Default|GetTotalRate))) ; レート合計値の1倍~0倍の数値を取得する
  (bind _outrownames_2 (DataTable|GetDataTableRowNames (Variables|Default|GetDropItemTable)))
  (for _array_element_2 _outrownames_2
    (bind _returnvalue_2 (Utilities|GetDataTableRow (Variables|Default|GetDropItemTable) _array_element_2)
      (:then
        (if (< (Variables|Default|GetRandomPoint) (.Rate (Utilities|Struct|BreakS_DropItem _returnvalue_2))) ; アイテムレートよりランダムポイントのレートが少ないか
          (return (.Type (Utilities|Struct|BreakS_DropItem _returnvalue_2)))
          (else
            (Variables|Default|SetRandomPoint (- (Variables|Default|GetRandomPoint) (.Rate (Utilities|Struct|BreakS_DropItem _returnvalue_2)))) ; ランダムポイントからそのアイテムのレートを引いて次ループの当選率を上げる
          ))))))