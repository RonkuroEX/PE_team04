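; Prototype shooter player built on a risk-reward loop of damage, including self-inflicted vaccine shots, and super recovery.
; Input drives swept movement, looping multi-way fire and a limited special attack granting brief invincibility.
; Lost HP debuffs movement and firing; after a delay, timed regeneration triggers one-shot milestone buffs scaled by damage severity, written into GI_PlayerStatus.
; Item pickups temporarily boost attack, speed or recovery, or add special charges.
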(event Custom|FireLoop
  (bind _proto_game_instance (Variables|Default|GetProto%20Game%20Instance))
  (bind _rightfrontpoint (Variables|Default|GetRightFrontPoint))
  (bind _returnvalue (Transformation|GetWorldLocation _rightfrontpoint))
  (bind _player_way (Variables|/Game/proto/Data/GI_PlayerStatus.GI_PlayerStatus_C|GetPlayer_Way _proto_game_instance))
  (bind _returnvalue_2 (Math|Float|Floor _player_way))
  ;[1 0.2869 0.2012] 弾の射撃
  (for _index (range 1 _returnvalue_2)
    (bind _returnvalue_3 (Game|SpawnActorfromClass "/Game/proto/BP/Player/BP_ProtoBullet.BP_ProtoBullet_C" (Math|Transform|MakeTransform (+ _returnvalue (* (/ (- (Transformation|GetWorldLocation (Variables|Default|GetLeftFrontPoint)) _returnvalue) (+ _returnvalue_2 1)) _index)) "0, 0, 0" "1.000000,1.000000,1.000000") "AlwaysSpawn" "MultiplyWithRoot" 0 0))
    (Default|GetBulletDamage _returnvalue_3 (* (Variables|/Game/proto/Data/GI_PlayerStatus.GI_PlayerStatus_C|GetPlayer_ATK (Variables|Default|GetProto%20Game%20Instance)) (Variables|バフ・デバフ|GetItemATKBuff_Volume)) (Variables|バフ・デバフ|GetDebuff_Volume))))

(event Custom|SuperRecovery
  (bind _proto_game_instance (Variables|Default|GetProto%20Game%20Instance))
  ;[0.17 1 0.1489] 一定時間後に超回復を発生させる
  (bind _returnvalue (Utilities|Time|SetTimerbyFunctionName 0 "カスタムイベント" 0.1 true))
  (Variables|タイマー|SetRecoveryTimer _returnvalue)
  (Variables|計算用|SetRiperdHP 0.0)
  (Variables|計算用|SetLostHP (- 1e+02 (Variables|ステータス|GetHP)))
  (Variables|計算用|SetFormerStatus (Utilities|Array|MakeArray (Variables|/Game/proto/Data/GI_PlayerStatus.GI_PlayerStatus_C|GetPlayer_ATK _proto_game_instance) (Variables|/Game/proto/Data/GI_PlayerStatus.GI_PlayerStatus_C|GetPlayer_speed _proto_game_instance) (Variables|/Game/proto/Data/GI_PlayerStatus.GI_PlayerStatus_C|GetPlayer_Way _proto_game_instance) (Variables|/Game/proto/Data/GI_PlayerStatus.GI_PlayerStatus_C|GetPlayer_FireDelay _proto_game_instance)))
  (Development|PrintString "回復開始！" true true "(R=0.000000,G=1.000000,B=0.117673,A=1.000000)"))

(event Custom|Debuff
  ;[1 0.225 0.9363] デバフ管理
  (CallFunction|CheckSeverityOfDamage)
  (Variables|バフ・デバフ|SetDebuff_Volume (Utilities|Select :Index (Variables|ステータス|GetSeverityDamage) :NewEnumerator0 0.0 :NewEnumerator1 0.25 :NewEnumerator2 0.5 :NewEnumerator3 0.75 :NewEnumerator4 0.9)))

(event Custom|カスタムイベント
  (Variables|計算用|SetRiperdHP (+ (Variables|計算用|GetRiperdHP) 1.0))
  (Variables|ステータス|SetHP (+ (Variables|ステータス|GetHP) 1.0))
  (CallFunction|Debuff)
  (Utilities|BuffCheck
    (:NewParam
      (if (>= (Variables|ステータス|GetHP) (Variables|/Game/proto/Data/GI_PlayerStatus.GI_PlayerStatus_C|GetPlayer_DefaultHP (Variables|Default|GetProto%20Game%20Instance)))
        (Variables|ステータス|SetHP (Variables|/Game/proto/Data/GI_PlayerStatus.GI_PlayerStatus_C|GetPlayer_DefaultHP (Variables|Default|GetProto%20Game%20Instance)))
        (Utilities|Time|ClearandInvalidateTimerbyHandle (Variables|タイマー|GetRecoveryTimer))
        (Development|PrintString "回復完了！" true true "(R=0.008359,G=1.000000,B=0.083694,A=1.000000)")))))

(event Custom|Recover
  (params (RecoveryTime :type Float%20%28double-precision%29))
  ;[0.17 1 0.1489] 一定時間後に超回復を発生させる
  (bind _returnvalue (Utilities|Time|SetTimerbyEvent (delegate Custom|SuperRecovery) RecoveryTime))
  (Variables|タイマー|SetRecoveryWaitTimer _returnvalue))

(event Input|EnhancedActionEvents|EnhancedInputActionIA_SPAttack
  (params (ActionValue :type Boolean) (ElapsedSeconds :type Float%20%28double-precision%29) (TriggeredSeconds :type Float%20%28double-precision%29) (InputAction :type Input%20Action%20Object%20Reference :default "/Game/proto/Input/Shooting/IA_SPAttack.IA_SPAttack"))
  (bind _spattackcount (Variables|ステータス|GetSPAttackCount))
  ;[1 0.1896 0.1916] 必殺技発動
  (Utilities|FlowControl|DoOnce false :!label _label
    (:Completed
      (if (> _spattackcount 0)
        (Math|Integer|DecrementInt _spattackcount
          (:%20%20
            (Variables|Default|Setinvincible true)
            (bind _returnvalue (Game|SpawnActorfromClass "/Game/proto/BP/Player/BP_ProtoSPAttack.BP_ProtoSPAttack_C" (Transformation|GetActorTransform) "Undefined" "MultiplyWithRoot" 0 0))
            (Default|SetDamage _returnvalue (Variables|/Game/proto/Data/GI_PlayerStatus.GI_PlayerStatus_C|GetPlayer_ATK (Variables|Default|GetProto%20Game%20Instance)))
            (Utilities|FlowControl|Delay 3.0)
            (Variables|Default|Setinvincible false)
            (goto _label Reset)))
        (else
          (Development|PrintString "必殺技の弾数が足りないです！" true true "(R=1.000000,G=0.000000,B=0.079394,A=1.000000)")
          (Utilities|FlowControl|Delay 3.0)
          (goto _label Reset))))))

(event Input|EnhancedActionEvents|EnhancedInputActionIA_Vaccine
  (params (ActionValue :type Boolean) (ElapsedSeconds :type Float%20%28double-precision%29) (TriggeredSeconds :type Float%20%28double-precision%29) (InputAction :type Input%20Action%20Object%20Reference :default "/Game/proto/Input/Shooting/IA_Vaccine.IA_Vaccine"))
  ;[1 0.2058 0.8832] ワクチン投与（自傷ダメージ）
  (:Started
    (if (Variables|Default|Getinvincible)
      (Development|PrintString "無敵状態でワクチンは使えなくなっています" true true "(R=1.000000,G=0.112500,B=0.112500,A=1.000000)")
      (else
        (Game|Damage|ApplyDamage self 25.0 0 0)
        (Development|PrintString "ワクチンを投与した")))))

(event Input|EnhancedActionEvents|EnhancedInputActionIA_Fire
  (params (ActionValue :type Float%20%28double-precision%29) (ElapsedSeconds :type Float%20%28double-precision%29) (TriggeredSeconds :type Float%20%28double-precision%29) (InputAction :type Input%20Action%20Object%20Reference :default "/Game/proto/Input/Shooting/IA_Fire.IA_Fire"))
  (bind _proto_game_instance (Variables|Default|GetProto%20Game%20Instance))
  (bind _player_firedelay (Variables|/Game/proto/Data/GI_PlayerStatus.GI_PlayerStatus_C|GetPlayer_FireDelay _proto_game_instance))
  ;[1 0.2869 0.2012] 弾の射撃
  (:Started
    (Variables|Default|SetCondition true)
    (Utilities|FlowControl|DoOnce false :!label _label
      (:Completed
        (if (Variables|Default|GetCondition) :!label _label_2
          (CallFunction|FireLoop)
          (Utilities|FlowControl|Delay (+ _player_firedelay (* _player_firedelay (Variables|バフ・デバフ|GetDebuff_Volume))))
          (goto _label_2)
          (else
            (goto _label Reset))))))
  (:Completed
    (Variables|Default|SetCondition false)))

(event Input|EnhancedActionEvents|EnhancedInputActionIA_move
  (params (ActionValue :type Vector%202D%20Structure) (ElapsedSeconds :type Float%20%28double-precision%29) (TriggeredSeconds :type Float%20%28double-precision%29) (InputAction :type Input%20Action%20Object%20Reference :default "/Game/proto/Input/Shooting/IA_move.IA_move"))
  (bind _itemspeedbuff_volume (Variables|バフ・デバフ|GetItemSpeedBuff_Volume))
  (bind _debuff_volume (Variables|バフ・デバフ|GetDebuff_Volume))
  (bind _proto_game_instance (Variables|Default|GetProto%20Game%20Instance))
  (bind _player_speed (Variables|/Game/proto/Data/GI_PlayerStatus.GI_PlayerStatus_C|GetPlayer_speed _proto_game_instance))
  (bind _returnvalue (* _player_speed _debuff_volume))
  (bind _returnvalue_2 (* _player_speed _itemspeedbuff_volume))
  (bind _returnvalue_3 (- _returnvalue_2 _returnvalue))
  ;[1 0.8292 0.3282] 上下左右移動
  (Transformation|SetActorLocation (+ (Transformation|GetActorLocation) (Math|Vector|NegateVector (Math|Vector|MakeVector (* (.x ActionValue) _returnvalue_3) (* (.y ActionValue) _returnvalue_3) 0.0))) true false))

(event Game|Damage|EventAnyDamage
  (params (Damage :type Float%20%28single-precision%29) (DamageType :type Damage%20Type%20Object%20Reference) (InstigatedBy :type Controller%20Object%20Reference) (DamageCauser :type Actor%20Object%20Reference))
  ;[1 0.2067 0.8354] 被ダメージ時の処理
  (if (not (Variables|Default|Getinvincible))
    (bind _output_get (Variables|ステータス|SetHP (- (Variables|ステータス|GetHP) Damage)))
    (if (<= _output_get 0.0)
      (Rendering|SetVisibility (Variables|Default|GetProtoPrayerBody) false false)
      (Variables|/Script/Engine.PrimitiveComponent|SetbGenerateOverlapEvents (Variables|Collision|GetCapsuleComponent) false)
      (Input|DisableInput 0)
      (Development|PrintString "GameOver" true true "(R=1.000000,G=0.000000,B=0.080609,A=1.000000)")
      (Utilities|Time|ClearandInvalidateTimerbyHandle (Variables|タイマー|GetRecoveryWaitTimer))
      (Variables|Default|SetCondition false)
      (else
        (Utilities|Time|ClearandInvalidateTimerbyHandle (Variables|タイマー|GetRecoveryTimer))
        (CallFunction|Debuff)
        (CallFunction|Recover (Variables|ステータス|GetRecoveryTime))))))

(event EventPossessed
  (params (NewController :type Controller%20Object%20Reference))
  (bind _asgi_player_status (Utilities|Casting|CastToGI_PlayerStatus (Game|GetGameInstance)))
  (bind _output_get (Variables|Default|SetProto%20Game%20Instance _asgi_player_status))
  (Variables|ステータス|SetHP (Variables|/Game/proto/Data/GI_PlayerStatus.GI_PlayerStatus_C|GetPlayer_DefaultHP _output_get))
  (bind _returnvalue (UserInterface|CreateWidget "/Game/proto/UI/PlayMenu/WBP_PlayMaster.WBP_PlayMaster_C"))
  (bind _output_get_2 (Variables|UI|SetWBP_PlayMaster _returnvalue))
  (UserInterface|Viewport|AddtoViewport _output_get_2 0))

(event EventIFFItemAdhibition
  (params (ItemType :type E_ItemType%20Enum :default "NewEnumerator0"))
  (bind _recoverywaittimer (Variables|タイマー|GetRecoveryWaitTimer))
  (bind _returnvalue (Utilities|Time|GetTimerRemainingTimebyHandle _recoverywaittimer))
  ;[1 0.4794 0.2048] アイテムの効果発動
  (switch Utilities|FlowControl|Switch|SwitchonE_ItemType ItemType
    (:NewEnumerator0
      (Variables|バフ・デバフ|SetItemATKBuff_Volume 1.5)
      (Development|PrintString "攻撃力1.5倍！！" true true "(R=1.000000,G=0.300000,B=0.900000,A=1.000000)")
      (Utilities|FlowControl|Delay 1e+01)
      (Variables|バフ・デバフ|SetItemATKBuff_Volume 1.0)
      (Development|PrintString "攻撃力が戻った" true true "(R=1.000000,G=0.300000,B=0.900000,A=1.000000)"))
    (:NewEnumerator1
      (Variables|バフ・デバフ|SetItemSpeedBuff_Volume 1.5)
      (Development|PrintString "移動速度1.5倍！！" true true "(R=1.000000,G=0.300000,B=0.900000,A=1.000000)")
      (Utilities|FlowControl|Delay 1e+01)
      (Variables|バフ・デバフ|SetItemSpeedBuff_Volume 1.0)
      (Development|PrintString "移動速度が戻った" true true "(R=1.000000,G=0.300000,B=0.900000,A=1.000000)"))
    (:NewEnumerator2
      (Variables|ステータス|SetRecoveryTime (/ (Variables|ステータス|GetRecoveryTime) 2.0))
      (Development|PrintString "回復時間半減！！" true true "(R=1.000000,G=0.300000,B=0.900000,A=1.000000)")
      (if (Utilities|Time|IsTimerActivebyHandle (Variables|タイマー|GetRecoveryWaitTimer))
        (CallFunction|Recover (/ _returnvalue 2.0))
        (Development|PrintString "現在のタイマーが半減した")
        (Development|PrintString (Utilities|String|ToString(Float) _returnvalue) true true "(R=1.000000,G=0.304280,B=0.950592,A=1.000000)"))
      (Utilities|FlowControl|Delay 1e+01)
      (Variables|ステータス|SetRecoveryTime (Utilities|GetClassDefaults "BP_ProtoPlayer1_C"))
      (Development|PrintString "回復時間が元に戻った" true true "(R=1.000000,G=0.300000,B=0.900000,A=1.000000)"))
    (:NewEnumerator3
      (Variables|ステータス|SetSPAttackCount (+ (Variables|ステータス|GetSPAttackCount) 1))
      (Development|PrintString "必殺技回数が増えた！！" true true "(R=1.000000,G=0.300000,B=0.900000,A=1.000000)"))))

(fn ConstructionScript)

(fn CheckSeverityOfDamage
  (bind _proto_game_instance (Variables|Default|GetProto%20Game%20Instance))
  (bind _player_defaulthp (Variables|/Game/proto/Data/GI_PlayerStatus.GI_PlayerStatus_C|GetPlayer_DefaultHP _proto_game_instance))
  (if (<= (Variables|ステータス|GetHP) (* _player_defaulthp 0.1))
    (Variables|ステータス|SetSeverityDamage "NewEnumerator4")
    (elif (<= (Variables|ステータス|GetHP) (* _player_defaulthp 0.25))
      (Variables|ステータス|SetSeverityDamage "NewEnumerator3")
      (elif (<= (Variables|ステータス|GetHP) (* _player_defaulthp 0.5))
        (Variables|ステータス|SetSeverityDamage "NewEnumerator2")
        (elif (<= (Variables|ステータス|GetHP) (* _player_defaulthp 0.75))
          (Variables|ステータス|SetSeverityDamage "NewEnumerator1")
          (else
            (Variables|ステータス|SetSeverityDamage "NewEnumerator0")))))))

(fn Buff*cal
  (params (Applicable%20to :type Float%20%28double-precision%29%20%28by%20ref%29) (FormerStatus :type Float%20%28double-precision%29))
  (|SetBy-RefVar Applicable%20to (* FormerStatus (Variables|バフ・デバフ|GetBuff_Volume))))

(fn Buff/cal
  (params (Applicable%20to :type Float%20%28double-precision%29%20%28by%20ref%29) (FormerStatus :type Float%20%28double-precision%29))
  (|SetBy-RefVar Applicable%20to (/ FormerStatus (Variables|バフ・デバフ|GetBuff_Volume))))

(fn BuffALLapply
  (CallFunction|Buff*cal (Variables|/Game/proto/Data/GI_PlayerStatus.GI_PlayerStatus_C|GetPlayer_ATK (Variables|Default|GetProto%20Game%20Instance)) (Utilities|Array|Get(acopy) (Variables|計算用|GetFormerStatus)))
  (CallFunction|Buff*cal (Variables|/Game/proto/Data/GI_PlayerStatus.GI_PlayerStatus_C|GetPlayer_speed (Variables|Default|GetProto%20Game%20Instance)) (Utilities|Array|Get(acopy) (Variables|計算用|GetFormerStatus) 1))
  (CallFunction|Buff*cal (Variables|/Game/proto/Data/GI_PlayerStatus.GI_PlayerStatus_C|GetPlayer_Way (Variables|Default|GetProto%20Game%20Instance)) (Utilities|Array|Get(acopy) (Variables|計算用|GetFormerStatus) 2))
  (CallFunction|Buff/cal (Variables|/Game/proto/Data/GI_PlayerStatus.GI_PlayerStatus_C|GetPlayer_FireDelay (Variables|Default|GetProto%20Game%20Instance)) (Utilities|Array|Get(acopy) (Variables|計算用|GetFormerStatus) 3)))

(fn BuffVolumeSet
  (params (Buff_Level :type Integer))
  (bind _lostseveritydamage (CallFunction|SetLostSeverityDamage))
  (LocalVariables|SetLostSeverityDamage _lostseveritydamage)
  (switch int Buff_Level ; 体力回復がどこまでいったかで分岐する\n1：50％以上\n2：75％以上\n3：90％以上\n4：完全回復
    (:1
      (Variables|バフ・デバフ|SetBuff_Volume (Utilities|Select :Index (LocalVariables|GetLostSeverityDamage) :NewEnumerator0 1.0 :NewEnumerator1 1.05 :NewEnumerator2 1.1 :NewEnumerator3 1.2 :NewEnumerator4 1.25)))
    (:2
      (Variables|バフ・デバフ|SetBuff_Volume (Utilities|Select :Index (LocalVariables|GetLostSeverityDamage) :NewEnumerator0 1.0 :NewEnumerator1 1.1 :NewEnumerator2 1.15 :NewEnumerator3 1.25 :NewEnumerator4 1.3)))
    (:3
      (Variables|バフ・デバフ|SetBuff_Volume (Utilities|Select :Index (LocalVariables|GetLostSeverityDamage) :NewEnumerator0 1.0 :NewEnumerator1 1.15 :NewEnumerator2 1.2 :NewEnumerator3 1.3 :NewEnumerator4 1.4)))
    (:4
      (Variables|バフ・デバフ|SetBuff_Volume (Utilities|Select :Index (LocalVariables|GetLostSeverityDamage) :NewEnumerator0 1.0 :NewEnumerator1 1.2 :NewEnumerator2 1.3 :NewEnumerator3 1.4 :NewEnumerator4 1.5))))
  (CallFunction|BuffALLapply))

(fn SetLostSeverityDamage
  (bind _proto_game_instance (Variables|Default|GetProto%20Game%20Instance))
  (bind _player_defaulthp (Variables|/Game/proto/Data/GI_PlayerStatus.GI_PlayerStatus_C|GetPlayer_DefaultHP _proto_game_instance))
  (if (<= (- 1e+02 (Variables|計算用|GetLostHP)) (* _player_defaulthp 0.1))
    (return "NewEnumerator4")
    (elif (<= (- 1e+02 (Variables|計算用|GetLostHP)) (* _player_defaulthp 0.25))
      (return "NewEnumerator3")
      (elif (<= (- 1e+02 (Variables|計算用|GetLostHP)) (* _player_defaulthp 0.5))
        (return "NewEnumerator2")
        (elif (<= (- 1e+02 (Variables|計算用|GetLostHP)) (* _player_defaulthp 0.75))
          (return "NewEnumerator1")
          (else
            (return "NewEnumerator0")))))))