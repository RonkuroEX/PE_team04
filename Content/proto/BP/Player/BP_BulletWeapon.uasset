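; Player bullet weapon that fires BP_ProtoBullet actors in one, three or five ways depending on WayLevel.
; IFFFire stores attack and way level, then a DoOnce reset after FireDelay limits the fire rate.
; FireLoop adds left/right muzzle pairs at levels 2 and 3.
; FSpawnBullet spawns at each muzzle's location, setting BaseDamage from the PlayerATK variable rather than its ATK input.
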(event Custom|FireLoop
  (CallFunction|FSpawnBullet (Variables|Default|Getmuzzle_Level1) (Variables|Default|GetPlayer%20ATK))
  (if (>= (Variables|Default|GetWay%20Level) 2)
    (CallFunction|FSpawnBullet (Variables|Default|Getmuzzle_Level2_Left) (Variables|Default|GetPlayer%20ATK))
    (CallFunction|FSpawnBullet (Variables|Default|Getmuzzle_Level2_Right) (Variables|Default|GetPlayer%20ATK))
    (if (>= (Variables|Default|GetWay%20Level) 3)
      (CallFunction|FSpawnBullet (Variables|Default|Getmuzzle_Level3_Left) (Variables|Default|GetPlayer%20ATK))
      (CallFunction|FSpawnBullet (Variables|Default|Getmuzzle_Level3_Right) (Variables|Default|GetPlayer%20ATK)))))

(event EventIFFFire
  (params (PlayerATK :type Float%20%28double-precision%29) (FireDelay :type Float%20%28double-precision%29) (WayLevel :type Integer))
  (Variables|Default|SetPlayer%20ATK PlayerATK)
  (Variables|Default|SetWay%20Level WayLevel)
  (Utilities|FlowControl|DoOnce false :!label _label
    (:Completed
      (CallFunction|FireLoop)
      (Utilities|FlowControl|Delay FireDelay)
      (goto _label Reset))))

(fn ConstructionScript)

(fn FSpawnBullet
  (params (muzzul :type Static%20Mesh%20Component%20Object%20Reference) (ATK :type Float%20%28double-precision%29))
  (Game|SpawnActorfromClass "/Game/proto/BP/Player/BP_ProtoBullet.BP_ProtoBullet_C" (Math|Transform|MakeTransform (Transformation|GetWorldLocation muzzul) "0, 0, 0" "1.000000,1.000000,1.000000") "AlwaysSpawn" "MultiplyWithRoot" 0 (Variables|Default|GetPlayer%20ATK) 0))