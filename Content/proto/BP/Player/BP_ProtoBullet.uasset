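; BP_ProtoBullet is a prototype player bullet actor that damages enemies on contact.
; GetBulletDamage sets BaseDamage from the player's attack plus that attack scaled by a debuff volume value.
; When the capsule begins overlapping an actor tagged Enemy, the bullet applies that damage, prints the amount for debugging and destroys itself.
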(event OnComponentBeginOverlap(Capsule)
  (params (OverlappedComponent :type Primitive%20Component%20Object%20Reference) (OtherActor :type Actor%20Object%20Reference) (OtherComp :type Primitive%20Component%20Object%20Reference) (OtherBodyIndex :type Integer) (bFromSweep :type Boolean) (SweepResult :type Hit%20Result%20Structure%20%28by%20ref%29))
  (bind _basedamage (Variables|Default|GetBaseDamage))
  (if (Actor|ActorHasTag OtherActor "Enemy")
    (Game|Damage|ApplyDamage OtherActor _basedamage 0 0)
    ;[1 1 1] デバッグ用
    (Development|PrintString (Utilities|String|Append "与えるダメージ：" (Utilities|String|ToString(Float) _basedamage)))
    (Actor|DestroyActor)))

(event Custom|GetBulletDamage
  (params (PlayerATK :type Float%20%28double-precision%29) (PlayerDebuffVolume :type Float%20%28double-precision%29))
  (Variables|Default|SetBaseDamage (+ PlayerATK (* PlayerATK PlayerDebuffVolume))))

(event EventTick
  (params (DeltaSeconds :type Float%20%28single-precision%29)))

(fn ConstructionScript)