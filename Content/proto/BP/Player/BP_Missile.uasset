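; BP_Missile is a player missile projectile that homes in on a target and damages enemies.
; On BeginPlay it sets a valid TargetActor's root component as the ProjectileMovement homing target.
; Capsule begin overlap with an "Enemy"-tagged actor applies BaseDamage, debug-prints the damage and destroys the missile.
; "Wall"-tagged actors destroy it only when the overlap ends, not on first contact.
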(event OnComponentBeginOverlap(Capsule)
  (params (OverlappedComponent :type Primitive%20Component%20Object%20Reference) (OtherActor :type Actor%20Object%20Reference) (OtherComp :type Primitive%20Component%20Object%20Reference) (OtherBodyIndex :type Integer) (bFromSweep :type Boolean) (SweepResult :type Hit%20Result%20Structure%20%28by%20ref%29))
  (if (Actor|ActorHasTag OtherActor "Enemy")
    (bind _returnvalue (Game|Damage|ApplyDamage OtherActor (Variables|Default|GetBaseDamage) 0 0))
    ;[1 1 1] デバッグ用
    (Development|PrintString (Utilities|String|Append "ミサイルの与えるダメージ：" (Utilities|String|ToString(Float) _returnvalue)))
    (Actor|DestroyActor)))

(event OnComponentEndOverlap(Capsule)
  (params (OverlappedComponent :type Primitive%20Component%20Object%20Reference) (OtherActor :type Actor%20Object%20Reference) (OtherComp :type Primitive%20Component%20Object%20Reference) (OtherBodyIndex :type Integer))
  (if (Actor|ActorHasTag OtherActor "Wall")
    (Actor|DestroyActor)))

(event EventBeginPlay
  (bind _targetactor (Variables|Default|GetTargetActor))
  (Utilities|IsValid _targetactor
    (:Is%20Valid
      (Development|PrintString (Utilities|GetDisplayName _targetactor))
      (Variables|/Script/Engine.ProjectileMovementComponent|SetHomingTargetComponent (Variables|Default|GetProjectileMovement) (Variables|/Script/Engine.Actor|GetRootComponent (Variables|Default|GetTargetActor))))))

(fn ConstructionScript)