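; BP_ProtoSPAttack1 is a prototype player special-attack bomb that damages actors overlapping its Box and destroys itself after five seconds.
; On BeginPlay it casts the game instance to GI_PlayerStatus and multiplies BaseDamage by PlayerATK to get the bomb damage.
; Each Box overlap applies that damage to the other actor without filtering and prints the result.
; The SetDamage event is an empty stub.
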(event OnComponentBeginOverlap(Box)
  (params (OverlappedComponent :type Primitive%20Component%20Object%20Reference) (OtherActor :type Actor%20Object%20Reference) (OtherComp :type Primitive%20Component%20Object%20Reference) (OtherBodyIndex :type Integer) (bFromSweep :type Boolean) (SweepResult :type Hit%20Result%20Structure%20%28by%20ref%29))
  (bind _returnvalue (Game|Damage|ApplyDamage OtherActor (Variables|Default|GetBomDanage) 0 0))
  (Development|PrintString (Utilities|String|ToString(Float) _returnvalue)))

(event Custom|SetDamage
  (params (PlayerATK :type Float%20%28double-precision%29)))

(event EventBeginPlay
  (bind _asgi_player_status (Utilities|Casting|CastToGI_PlayerStatus (Game|GetGameInstance)))
  (bind _output_get (Variables|Default|SetProto%20Game%20Instance _asgi_player_status))
  (Variables|Default|SetBomDanage (* (Variables|Default|GetBaseDamage) (Variables|/Game/proto/Data/GI_PlayerStatus.GI_PlayerStatus_C|GetPlayer_ATK _output_get))) ; ベースダメージ×プレイヤーの攻撃力が最終的なボムのダメージになります
  (Utilities|FlowControl|Delay 5.0)
  (Actor|DestroyActor))

(fn ConstructionScript)